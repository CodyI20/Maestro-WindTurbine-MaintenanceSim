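; BP_MiniTurbine is a miniature figure that displays either a drone scavenger or a mannequin on a colored ground piece.
; The Construction Script uses the IsDroneLevel flag to show one figure and hide the other.
; The same flag sets the ground material to green for drone levels and blue otherwise.
; The Event Graph holds only empty default events, so the actor has no runtime logic of its own.
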(event EventBeginPlay)

(event Collision|EventActorBeginOverlap
  (params (OtherActor :type Actor%20Object%20Reference)))

(event EventTick
  (params (DeltaSeconds :type Float%20%28single-precision%29)))

(fn ConstructionScript
  (bind _isdronelevel (Variables|Default|GetIsDroneLevel))
  (Rendering|SetVisibility (Variables|Default|GetSK_Drone_Scavenger) _isdronelevel false)
  (Rendering|SetVisibility (Variables|Default|GetSK_Mannequin) (not _isdronelevel) false)
  (if _isdronelevel
    (Rendering|Material|SetMaterial (Variables|Default|GetGround) 0 "/Game/Miniture_Figures/M_Green_MiniShape.M_Green_MiniShape")
    (else
      (Rendering|Material|SetMaterial (Variables|Default|GetGround) 0 "/Game/Miniture_Figures/M_Blue_MiniShape.M_Blue_MiniShape"))))