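; BP_Menu is a menu Blueprint with laser-pointer helpers for pointing at widgets through Widget Interaction components.
; On BeginPlay it calls an empty event-subscription stub and, a tick later, enables input and adds the menu mapping context.
; UpdateLaserAndCursor, not called here, toggles laser and cursor visibility and feeds the Niagara beam's endpoints through a point array.
; Laser color setup is disconnected, and SetWidgetInteractionReference is empty.
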(event EventBeginPlay
  (bind _returnvalue (Game|GetPlayerController 0))
  (Utilities|FlowControl|Sequence
    (:then_0
      (CallFunction|SubscribetoEvents))
    (:then_1
      (Utilities|FlowControl|DelayUntilNextTick)
      (Input|EnableInput _returnvalue)
      (Input|AddMappingContext (PlayerController|LocalPlayerSubsystems|GetEnhancedInputLocalPlayerSubsystem _returnvalue) "/Game/VRTemplate/Input/IMC_Menu.IMC_Menu" 0 "(bIgnoreAllPressedKeysUntilRelease=True,bForceImmediately=False,bNotifyUserSettings=False)"))))

(event Custom|SubscribeToEvents)

(fn ConstructionScript)

(fn SetWidgetInteractionReference)

(fn UpdateLaserandCursor
  (params (LasrerAlwaysVisible :type Boolean) (WidgetInteractionComponent :type Widget%20Interaction%20Component%20Object%20Reference) (Cursor :type Static%20Mesh%20Component%20Object%20Reference) (Laser :type Niagara%20Component%20Object%20Reference))
  (if (or LasrerAlwaysVisible (Class|WidgetInteractionComponent|IsOverHitTestVisibleWidget WidgetInteractionComponent))
    (CallFunction|LaserCursorVisibility true Laser Cursor)
    (Variables|Default|SetLaserStartPoint (Transformation|GetWorldLocation WidgetInteractionComponent))
    (if (Class|WidgetInteractionComponent|IsOverHitTestVisibleWidget WidgetInteractionComponent)
      (Variables|Default|SetLaserEndPoint (|GetLastHitResultCollapsed WidgetInteractionComponent))
      (Transformation|SetWorldLocation Cursor (Variables|Default|GetLaserEndPoint) false false)
      (else
        (Variables|Default|SetLaserEndPoint (|FindEndofWidgetInteractionComponent WidgetInteractionComponent))
        (Rendering|SetVisibility Cursor false false)))
    (Class|NiagaraDataInterfaceArrayFunctionLibrary|SetNiagaraArrayVectorValue Laser "User.PointArray" 0 (Variables|Default|GetLaserStartPoint) false)
    (Class|NiagaraDataInterfaceArrayFunctionLibrary|SetNiagaraArrayVectorValue Laser "User.PointArray" 1 (Variables|Default|GetLaserEndPoint) false)
    (else
      (CallFunction|LaserCursorVisibility false Laser Cursor))))

(fn LaserCursorVisibility
  (params (Visibility :type Boolean) (Laser :type Niagara%20Component%20Object%20Reference) (Cursor :type Static%20Mesh%20Component%20Object%20Reference))
  (Rendering|SetVisibility Laser Visibility false)
  (Rendering|SetVisibility Cursor Visibility false))