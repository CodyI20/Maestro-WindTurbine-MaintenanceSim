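; BP_Select is a menu selection actor that displays a Select_Menu_FP widget through a widget component.
; On BeginPlay it casts that widget, passes it the actor's BackgroundColor and calls SetBeginColor to apply the starting color.
; Tick and overlap events are disabled, and the construction script only calls its parent, so all other behavior lives in the widget or parent class.
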(event EventBeginPlay
  (|CallParentFunction)
  (bind _asselect_menu_fp (Utilities|Casting|CastToSelect_Menu_FP (UserInterface|GetWidget (Variables|Default|GetWidget))))
  (Variables|/Game/Menu/Select_Menu_FP.Select_Menu_FP_C|SetColor _asselect_menu_fp (Variables|Default|GetBackgroundColor))
  (Default|SetBeginColor _asselect_menu_fp))

(event Collision|EventActorBeginOverlap
  (params (OtherActor :type Actor%20Object%20Reference))
  (|CallParentFunction OtherActor) ; This node is disabled and will not be called.\nDrag off pins to build functionality.
)

(event EventTick
  (params (DeltaSeconds :type Float%20%28single-precision%29))
  (|CallParentFunction DeltaSeconds) ; This node is disabled and will not be called.\nDrag off pins to build functionality.
)

(fn ConstructionScript
  (|CallParentFunction))