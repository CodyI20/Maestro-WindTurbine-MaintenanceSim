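; Handheld menu actor that shows or hides a widget menu through the menu toggle input.
; On BeginPlay it hides itself, caches the Settings_Menu widget and binds its warning confirmation, which hides the menu.
; Toggling with changed settings raises that warning instead; otherwise root visibility flips and widget collision follows, so the hidden menu blocks nothing.
; A Main_Menu start button, if that widget is present, toggles visibility only, without updating collision.
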(event Custom|WarningMenuYesButtonPressed_Event
  (CallFunction|MenuInteractabilityLogic false))

(event Input|EnhancedActionEvents|EnhancedInputActionIA_Menu_Toggle
  (params (ActionValue :type Boolean) (ElapsedSeconds :type Float%20%28double-precision%29) (TriggeredSeconds :type Float%20%28double-precision%29) (InputAction :type Input%20Action%20Object%20Reference :default "/Game/VRTemplate/Input/Actions/IA_Menu_Toggle.IA_Menu_Toggle"))
  ;[0.15 0.15 0.15 0.5] Toggle handheld menu
  (if (Variables|/Game/Menu/Settings_Menu.Settings_Menu_C|GetIsSettingsChanged (Variables|Default|GetSettings%20Menu))
    (Default|SetWarningMenuVisibility (Variables|Default|GetSettings%20Menu) "Visible" false)
    (else
      (CallFunction|MenuInteractabilityLogic true))))

(event EventBeginPlay
  (|CallParentFunction)
  (Utilities|FlowControl|Sequence
    (:then_0
      (|StartButtonPressMainMenu))
    (:then_1
      (|InitMenu))
    (:then_2
      (|Getsettingsmenufromwidget))
    (:then_3
      (EventDispatchers|AssignWarningMenuYesButtonPressed (Variables|Default|GetSettings%20Menu) (delegate Custom|WarningMenuYesButtonPressed_Event)))))

(event Collision|EventActorBeginOverlap
  (params (OtherActor :type Actor%20Object%20Reference))
  (|CallParentFunction OtherActor) ; This node is disabled and will not be called.\nDrag off pins to build functionality.
)

(event EventTick
  (params (DeltaSeconds :type Float%20%28single-precision%29))
  (|CallParentFunction DeltaSeconds) ; This node is disabled and will not be called.\nDrag off pins to build functionality.
)

(fn ConstructionScript
  (|CallParentFunction))

(fn MenuInteractabilityLogic
  (params (isToggle :type Boolean))
  (if isToggle
    (Rendering|ToggleVisibility (Variables|Default|GetDefaultSceneRoot) true)
    (else
      (Rendering|SetVisibility (Variables|Default|GetDefaultSceneRoot) false true)))
  ;[0.15 0.15 0.15 0.5] Make the menu non-interactable/non-obstructive while invisible
  (if (Rendering|IsVisible (Variables|Default|GetDefaultSceneRoot))
    (Collision|SetCollisionResponsetoAllChannels (Variables|Default|GetWidget) "ECR_Block")
    (else
      (Collision|SetCollisionResponsetoAllChannels (Variables|Default|GetWidget) "ECR_Ignore"))))

(event Custom|StartButtonPressed_Event
  (Rendering|ToggleVisibility (Variables|Default|GetDefaultSceneRoot) true))