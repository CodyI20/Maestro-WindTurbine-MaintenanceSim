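; Physics-simulated rope actor with configurable length and link count, drawn as a smooth spline mesh.
; Construction builds a chain of static mesh links joined by physics constraints, with only the first link non-simulated as an anchor.
; These links are physics reference points: every Tick, spline points follow them and spline mesh segments are re-fitted along the curve.
; The grab-related damping functions are stubs with disconnected logic.
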(event EventTick
  (params (DeltaSeconds :type Float%20%28single-precision%29))
  (CallFunction|UpdateSpline))

(event EventBeginPlay
  (Variables|Default|SetRopeSegmentLength (/ (Variables|Default|GetRopeLength) (Variables|Default|GetNumLinks)))
  (CallFunction|AdjustPhysicsConstraints)
  (Components|MoveComponentTo (Utilities|Array|Get(acopy) (Variables|Default|GetLinks)) "0.000000,0.000000,0.000000" "0, 0, 0" false false 0.2 false))

(fn ConstructionScript
  (CallFunction|RopeInnit))

(fn UpdateSpline
  (bind _spline (Variables|Default|GetSpline))
  (bind _spline_2 (Variables|Default|GetSpline))
  (Utilities|FlowControl|Sequence
    (:then_0
      (for (_array_element _array_index) (Variables|Default|GetLinks)
        (Spline|SetLocationatSplinePoint (Variables|Default|GetSpline) _array_index (Transformation|GetWorldLocation _array_element) "World" true)))
    (:then_1
      (for (_array_element_2 _array_index_2) (Variables|Default|GetSplineMeshSegments)
        (SplineMesh|SetStartandEnd _array_element_2 (Spline|GetLocationatDistanceAlongSpline _spline_2 (* _array_index_2 (Variables|Default|GetRopeSegmentLength)) "Local") (Spline|GetTangentatDistanceAlongSpline _spline_2 (* _array_index_2 (Variables|Default|GetRopeSegmentLength)) "Local") (Spline|GetLocationatDistanceAlongSpline _spline (* (+ _array_index_2 1) (Variables|Default|GetRopeSegmentLength)) "Local") (Spline|GetTangentatDistanceAlongSpline _spline (* (+ _array_index_2 1) (Variables|Default|GetRopeSegmentLength)) "Local") true :!class /Script/Engine.SplineMeshComponent)))))

(fn AdjustPhysicsConstraints
  (for _array_element (Variables|Default|GetLinks)
    (bind _returnvalue (Physics|GetPhysicsLinearVelocity _array_element "None"))
    (Physics|SetPhysicsLinearVelocity _array_element (Math|Vector|MakeVector (.X (Math|Vector|BreakVector _returnvalue)) (.Y (Math|Vector|BreakVector _returnvalue)) 0.0) false "None")))

(fn ActivateDampingSettings
  (params (GrabbedIndex :type Integer)))

(fn DeactivateDampingSettings)

(fn RopeInnit
  (bind _links (Variables|Default|GetLinks))
  (LocalVariables|SetAdjMeshLength (/ (Variables|Default|GetRopeLength) (Variables|Default|GetNumLinks)))
  (for _index (range 0 (- (Variables|Default|GetNumLinks) 1))
    (Utilities|FlowControl|Sequence
      (:then_0
        ;[0.15 0.15 0.15 0.5] Add static meshes and set simulate physics for all, but the first component added. This however is not the visible mesh itself, but rather a physics reference point
        (bind _returnvalue (AddComponent|AddStaticMeshComponent false))
        (Physics|SetSimulatePhysics _returnvalue (!= 0 _index))
        (Transformation|AttachComponentToComponent _returnvalue (Variables|Default|GetSpline) "None" "KeepWorld" "KeepWorld" "KeepWorld" false)
        (Transformation|SetRelativeLocation _returnvalue (Math|Vector|MakeVector (Math|Conversions|ToFloat(Integer) (* _index (LocalVariables|GetAdjMeshLength))) 0.0 0.0) false false)
        (Utilities|Array|Add (Variables|Default|GetLinks) _returnvalue)
        (Utilities|Map|Add (Variables|Default|GetLinkIndexes) _returnvalue _index))
      (:then_1
        ;[0.15 0.15 0.15 0.5] Add physics constraint to every added static mesh. This is what makes the rope behaviour work
        (bind _returnvalue_2 (AddComponent|AddPhysicsConstraintComponent false))
        (Transformation|SetRelativeLocation _returnvalue_2 (Math|Vector|MakeVector (Math|Conversions|ToFloat(Integer) (* _index (LocalVariables|GetAdjMeshLength))) 0.0 0.0) false false)
        (if (!= 0 _index)
          (Class|PhysicsConstraintComponent|SetConstrainedComponents _returnvalue_2 (Utilities|Array|Get(acopy) _links (- _index 1)) "None" (Utilities|Array|Get(acopy) _links _index) "None"))
        (Utilities|Array|Add (Variables|Default|GetConstraints) _returnvalue_2))))
  ;[0.15 0.15 0.15 0.5] Reset spline and add all points with a cylinder mesh. This handles the visual part of the rope, connecting it smoothly
  (Spline|ClearSplinePoints (Variables|Default|GetSpline) true)
  (for _array_element (Variables|Default|GetLinks)
    (Spline|AddSplinePoint (Variables|Default|GetSpline) (Transformation|GetWorldLocation _array_element) "World" true)
    (bind _returnvalue_3 (AddComponent|AddSplineMeshComponent false))
    (Rendering|Material|SetMaterial _returnvalue_3 0 "/Game/Materials/Rope/M_Rope.M_Rope")
    (Transformation|AttachComponentToComponent _returnvalue_3 (Variables|Default|GetSpline) "None" "KeepRelative" "KeepRelative" "KeepRelative" false)
    (Utilities|Array|Add (Variables|Default|GetSplineMeshSegments) _returnvalue_3)))