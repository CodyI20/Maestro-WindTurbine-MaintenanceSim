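; Base actor for interactive miniature turbines that highlight on hover and toggle a BP_Select child-actor panel when interacted with.
; BeginPlay caches child static and skeletal meshes with custom depth enabled, toggles the panel once, and gathers all turbine actors.
; Hover events switch the meshes' stencil values to drive the highlight.
; Interaction force-closes other turbines' panels and toggles its own visibility and widget collision.
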(event EventBeginPlay
  (bind _defaultsceneroot (Variables|Default|GetDefaultSceneRoot))
  (bind _children (Components|GetChildrenComponents _defaultsceneroot false))
  (Utilities|FlowControl|Sequence
    (:then_0
      (for _array_element _children
        (bind _asstatic_mesh_component (Utilities|Casting|CastToStaticMeshComponent _array_element))
        (Utilities|Array|AddUnique (Variables|Default|GetStaticMeshComponents) _asstatic_mesh_component)
        (Rendering|SetRenderCustomDepth _asstatic_mesh_component true)))
    (:then_1
      (for _array_element_2 _children
        (bind _asskeletal_mesh_component (Utilities|Casting|CastToSkeletalMeshComponent _array_element_2))
        (Utilities|Array|AddUnique (Variables|Default|GetSkeletalMeshComponents) _asskeletal_mesh_component)
        (Rendering|SetRenderCustomDepth _asskeletal_mesh_component true)))
    (:then_2
      (CallFunction|ToggleVisibilityBPSelect))
    (:then_3
      (bind _outactors (Actor|GetAllActorsOfClass "BP_MiniTurbineBASE_C"))
      (Variables|Default|SetMiniTurbineActors _outactors))))

(event EventOnBeginHover
  (CallFunction|SetMeshStencilValue 1))

(event EventOnEndHover
  (CallFunction|SetMeshStencilValue))

(event EventOnInteracted
  (bind _miniturbineactors (Variables|Default|GetMiniTurbineActors))
  (if (> (Utilities|Array|Length _miniturbineactors) 0)
    (for _array_element _miniturbineactors
      (if (!= _array_element self)
        (CallFunction|ForceClosePanel _array_element)
        (else
          (CallFunction|ToggleVisibilityBPSelect))))))

(fn ConstructionScript)

(fn ToggleOutline
  (params (Active? :type Boolean))
  (bind _ground (Variables|Default|GetGround))
  (Rendering|SetRenderCustomDepth _ground Active?)
  (Rendering|SetCustomDepthStencilValue _ground (Math|Integer|SelectInt 1 0 Active?)))

(fn SetMeshStencilValue
  (params (StencilValue :type Integer))
  (Utilities|FlowControl|Sequence
    (:then_0
      (for _array_element (Variables|Default|GetStaticMeshComponents)
        (Rendering|SetCustomDepthStencilValue _array_element StencilValue)))
    (:then_1
      (for _array_element_2 (Variables|Default|GetSkeletalMeshComponents)
        (Rendering|SetCustomDepthStencilValue _array_element_2 StencilValue)))))

(fn ToggleVisibilityBPSelect
  (bind _bp_select (Variables|Default|GetBP_Select))
  (bind _bp_select_2 (Variables|Default|GetBP_Select)
    (:then
      (Components|Activation|ToggleActive _bp_select_2)
      (Rendering|ToggleVisibility _bp_select_2 true)
      (bind _asbp_select (Utilities|Casting|CastToBP_Select (Variables|/Script/Engine.ChildActorComponent|GetChildActor _bp_select)))
      (Default|ToggleWidgetCollision _asbp_select (Variables|/Script/Engine.SceneComponent|GetbVisible _bp_select)))
    (:else)))

(fn ForceClosePanel
  (bind _bp_select (Variables|Default|GetBP_Select))
  (Components|Activation|SetActive _bp_select false false)
  (Rendering|SetVisibility _bp_select false true))