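; BP_OffShorePlacer lays out offshore wind turbine instances in a rectangular grid, built in the construction script.
; Nested loops over WidthHeight step a running transform by DistanceBetweenInstance, resetting local Y after each row.
; Each cell adds the same transform to two instanced static mesh components, except one hard-coded grid cell that is left empty.
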(fn ConstructionScript
  (bind _widthheight (Variables|Default|GetWidthHeight))
  (bind (_x _y) (Utilities|Struct|BreakIntVector2 _widthheight))
  (for _index (range 0 (- _x 1))
    (for _index_2 (range 0 (- _y 1))
      (if (and (== (.x (Variables|Default|GetCurrentWidthHeight)) 2) (== (.y (Variables|Default|GetCurrentWidthHeight)) 4))
        _
        (else
          (Components|InstancedStaticMesh|AddInstance (Variables|Default|GetInstancedStaticMesh) (Variables|Default|GetCurrentTransform) false)
          (Components|InstancedStaticMesh|AddInstance (Variables|Default|GetInstancedStaticMesh1) (Variables|Default|GetCurrentTransform) false)))
      (Variables|Default|SetCurrentTransform (Math|Transform|MakeTransform (+ (.location (Variables|Default|GetCurrentTransform)) (Math|Vector|MakeVector 0.0 (.y (Variables|Default|GetDistanceBetweenInstance)) 0.0)) "0, 0, 0" "1.000000,1.000000,1.000000"))
      (Variables|Default|SetCurrentWidthHeight (Utilities|Struct|MakeIntVector2 (+ (.x (Variables|Default|GetCurrentWidthHeight)) 1) (.y (Variables|Default|GetCurrentWidthHeight)))))
    (Variables|Default|SetCurrentTransform (Math|Transform|MakeTransform (+ (.location (Variables|Default|GetCurrentTransform)) (Math|Vector|MakeVector (.x (Variables|Default|GetDistanceBetweenInstance)) (* (.y (.location (Variables|Default|GetCurrentTransform))) -1.0) 0.0)) "0, 0, 0" "1.000000,1.000000,1.000000"))
    (Variables|Default|SetCurrentWidthHeight (Utilities|Struct|MakeIntVector2 0 (+ (.y (Variables|Default|GetCurrentWidthHeight)) 1)))))