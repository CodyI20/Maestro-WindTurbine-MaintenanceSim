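; Outline handler component that highlights a mesh once the VR character or drone has stayed inside a sphere collider for a set time.
; Setup supplies mesh, collider and delay, while overlap events and a first-tick overlap check toggle the timer advanced on Tick.
; The outline uses custom depth stencil, clears on exit, and reappears without delay after its first activation.
; The component can be activated or deactivated; the overlay material path is unused.
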(event Custom|OnComponentBeginOverlap_Event
  (params (OverlappedComponent :type Primitive%20Component%20Object%20Reference) (OtherActor :type Actor%20Object%20Reference) (OtherComp :type Primitive%20Component%20Object%20Reference) (OtherBodyIndex :type Integer) (bFromSweep :type Boolean) (SweepResult :type Hit%20Result%20Structure%20%28by%20ref%29))
  ;[0.15 0.15 0.15 0.5] Assign collision events to timer toggle
  (Utilities|Casting|CastToVRCharacter OtherActor
    (:then
      _)
    (:CastFailed
      (Utilities|Casting|CastToBP_Drone OtherActor)))
  (CallFunction|StartTimer))

(event Custom|OnComponentEndOverlap_Event
  (params (OverlappedComponent :type Primitive%20Component%20Object%20Reference) (OtherActor :type Actor%20Object%20Reference) (OtherComp :type Primitive%20Component%20Object%20Reference) (OtherBodyIndex :type Integer))
  ;[0.15 0.15 0.15 0.5] Assign collision events to timer toggle
  (Utilities|Casting|CastToVRCharacter OtherActor
    (:then
      _)
    (:CastFailed
      (Utilities|Casting|CastToBP_Drone OtherActor)))
  (CallFunction|StopTimer))

(event Custom|SetupColEvents
  (bind _spherecollider (Variables|Default|GetSphereCollider))
  ;[0.15 0.15 0.15 0.5] Assign collision events to timer toggle
  (Collision|AssignOnComponentBeginOverlap _spherecollider (delegate Custom|OnComponentBeginOverlap_Event))
  (Collision|AssignOnComponentEndOverlap _spherecollider (delegate Custom|OnComponentEndOverlap_Event)))

(event EventTick
  (params (DeltaSeconds :type Float%20%28single-precision%29))
  (Utilities|FlowControl|Sequence
    (:then_0
      ;[0.15 0.15 0.15 0.5] Activate Outline, if player is already inside the collider on spawn
      (Utilities|FlowControl|DoOnce false
        (:Completed
          (for _array_element (Collision|GetOverlappingActors (Variables|Default|GetSphereCollider) 0 :!class /Script/Engine.PrimitiveComponent)
            (Utilities|Casting|CastToBP_VRCharacter _array_element
              (:then
                _)
              (:CastFailed
                (Utilities|Casting|CastToBP_Drone _array_element)))
            (CallFunction|StartTimer)))))
    (:then_1
      (if (Variables|Default|GetComponentActive)
        (CallFunction|UpdateTime DeltaSeconds)))))

(fn StartTimer
  ;[0.15 0.15 0.15 0.5] Activate timer
  (Variables|Default|SetIsTimerActive true))

(fn StopTimer
  (bind _meshtooutline (Variables|Default|GetMeshToOutline))
  ;[0.15 0.15 0.15 0.5] Reset timer/values and remove outline
  (Variables|Default|SetIsTimerActive false)
  (Variables|Default|SetIsOutlineActive false)
  (Variables|Default|SetTimePassed 0.0)
  (Rendering|SetRenderCustomDepth _meshtooutline false)
  (Rendering|SetCustomDepthStencilValue _meshtooutline 0))

(fn UpdateTime
  (params (deltaTime :type Float%20%28double-precision%29))
  (bind _meshtooutline (Variables|Default|GetMeshToOutline))
  ;[0.15 0.15 0.15 0.5] Run timer when active, and activate when complete and outline is not yet active
  (if (Math|Boolean|ANDBoolean (Variables|Default|GetWasActivated) (not (Variables|Default|GetIsOutlineActive)) (Variables|Default|GetIsTimerActive))
    ;[0.15 0.15 0.15 0.5] Apply outline
    (Variables|Default|SetIsOutlineActive true :!label _label)
    (Rendering|SetRenderCustomDepth _meshtooutline true)
    (Rendering|SetCustomDepthStencilValue _meshtooutline 1)
    (Variables|Default|SetWasActivated true)
    (elif (Variables|Default|GetIsTimerActive)
      (bind _output_get (Variables|Default|SetTimePassed (+ deltaTime (Variables|Default|GetTimePassed))))
      (if (and (> _output_get (Variables|Default|GetOutlineTime)) (not (Variables|Default|GetIsOutlineActive)))
        (goto _label)))))

(fn Setup
  (params (StaticMesh :type Static%20Mesh%20Component%20Object%20Reference) (SphereCollider :type Sphere%20Component%20Object%20Reference) (OutlineMaterialInstance :type Material%20Instance%20Object%20Reference) (OutlineTime :type Float%20%28double-precision%29))
  ;[0.15 0.15 0.15 0.5] Setup collider & the mesh to be outlined
  (Variables|Default|SetMeshToOutline StaticMesh)
  (Variables|Default|SetSphereCollider SphereCollider)
  (CallFunction|SetupColEvents)
  (Variables|Default|SetOutlineTime OutlineTime)
  (Variables|Default|SetOutlineMaterial OutlineMaterialInstance))

(fn DeactivateComponent
  (bind _meshtooutline (Variables|Default|GetMeshToOutline))
  (CallFunction|StopTimer)
  (Variables|Default|SetComponentActive false)
  (Rendering|SetRenderCustomDepth _meshtooutline false)
  (Rendering|SetCustomDepthStencilValue _meshtooutline 0))

(fn ActivateComponent
  (Variables|Default|SetComponentActive true))