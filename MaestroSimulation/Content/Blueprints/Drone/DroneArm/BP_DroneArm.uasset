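; BP_DroneArm is a drone's robot arm carrying a bristle tool, steered by the VR player's left motion controller while the drone is taken over.
; Setup wires the bristle and paint components and attaches the inner mesh to the arm socket; SetActivataion toggles the bristles.
; While active, Tick feeds the offset controller position and bristle rotation into ABP_RobotArm.
; Physical animation simulates the bones below the chain's first bone.
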(event EventBeginPlay
  (bind _physicalanimation (Variables|Default|GetPhysicalAnimation))
  (Class|PhysicalAnimationComponent|SetSkeletalMeshComponent _physicalanimation (Variables|Default|GetRobotMesh))
  (Class|PhysicalAnimationComponent|ApplyPhysicalAnimationSettingsBelow _physicalanimation (Variables|Default|GetFirstBoneInChainName) (Utilities|Struct|MakePhysicalAnimationData true 2e+03 1e+02 1e+03 1e+02) false)
  (Class|SkeletalMeshComponent|SetAllBodiesBelowSimulatePhysics (Variables|Default|GetRobotMesh) (Variables|Default|GetFirstBoneInChainName) true false)
  (CallFunction|Setup))

(event EventOnTakenOverEnd
  (Variables|Default|SetbIsActive false))

(event EventOnTakenOverBegin
  (Variables|Default|SetbIsActive true))

(event EventTick
  (params (DeltaSeconds :type Float%20%28single-precision%29))
  (Utilities|FlowControl|Sequence
    (:then_0
      (Utilities|FlowControl|DoOnce false
        (:Completed
          (bind _asabp_robot_arm (Utilities|Casting|CastToABP_RobotArm (Components|SkeletalMesh|GetAnimInstance (Variables|Default|GetRobotMesh))))
          (Variables|Default|SetRobotArmAnimBP _asabp_robot_arm))))
    (:then_1
      (CallFunction|UpdateDrone))))

(fn ConstructionScript)

(fn Setup
  (Default|Setup (Variables|Default|GetBP_BristleComponent) (Variables|Default|GetInnerStaticMesh) (Variables|Default|GetOuterStaticMesh) 0 0 (Variables|Default|GetBP_PaintComponent) true (Variables|Default|GetBristleSound))
  ;[0.15 0.15 0.15 0.5] Get Animation Blueprint of Skeletal Mesh
  (bind _asabp_robot_arm (Utilities|Casting|CastToABP_RobotArm (Components|SkeletalMesh|GetAnimInstance (Variables|Default|GetRobotMesh))))
  (Variables|Default|SetRobotArmAnim _asabp_robot_arm)
  (Transformation|AttachComponentToComponent (Variables|Default|GetInnerStaticMesh) (Variables|Default|GetRobotMesh) "do_touch" "KeepRelative" "KeepRelative" "KeepRelative" true))

(fn UpdateAnimation
  (bind _robotarmanimbp (Variables|Default|GetRobotArmAnimBP)
    (:then
      (Variables|/Game/Drone/ArmProperUVs/ABP_RobotArm.ABP_RobotArm_C|SetBlasterRotation _robotarmanimbp (Variables|/Game/Blueprints/BristleBlaster/BP_BristleBlaster_Handler.BP_BristleBlaster_Handler_C|GetCurrentBristleRotation (Variables|Default|GetBP_BristleComponent))))
    (:else)))

(fn ControlArm
  ;[0.15 0.001186 0 0.5 10] TEMPORARY FIX FOR STANDALONE WINDOW
  (bind _ascustom_vrcharacter (Utilities|Casting|CastToCustom_VRCharacter (Game|Player|GetPlayerPawn 0)))
  (Variables|/Game/Drone/ArmProperUVs/ABP_RobotArm.ABP_RobotArm_C|SetFinalTransform (Variables|Default|GetRobotArmAnimBP) (Math|Transform|MakeTransform (Math|Vector|MakeVector (+ (.x (.location (Transformation|GetRelativeTransform (Variables|/Script/VRExpansionPlugin.VRBaseCharacter|GetLeftMotionController _ascustom_vrcharacter)))) 35.0) (+ (.y (.location (Transformation|GetRelativeTransform (Variables|/Script/VRExpansionPlugin.VRBaseCharacter|GetLeftMotionController _ascustom_vrcharacter)))) 1e+01) (- (.z (.location (Transformation|GetRelativeTransform (Variables|/Script/VRExpansionPlugin.VRBaseCharacter|GetLeftMotionController _ascustom_vrcharacter)))) (.z (Variables|Default|GetControllerOffset)))))))

(fn UpdateDrone
  (if (Variables|Default|GetbIsActive)
    (CallFunction|ControlArm)
    (CallFunction|UpdateAnimation)))

(fn SetActivataion
  (params (Activate :type Boolean))
  (bind _bp_bristlecomponent (Variables|Default|GetBP_BristleComponent))
  (if Activate
    (Default|Turnon _bp_bristlecomponent)
    (else
      (Default|TurnOff _bp_bristlecomponent))))