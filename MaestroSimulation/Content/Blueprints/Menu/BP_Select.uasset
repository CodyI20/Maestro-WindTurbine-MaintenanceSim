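; BP_Select is a menu actor that hosts a WBP_Select_Menu_FP selection menu in its widget component.
; On BeginPlay it caches the menu widget and passes in its own level type and hovered and unhovered colors.
; ToggleWidgetCollision switches the widget component between query-only and no collision according to a visibility flag.
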(event EventBeginPlay
  (|CallParentFunction)
  (bind _asselect_menu_fp (Utilities|Casting|CastToWBP_Select_Menu_FP (UserInterface|GetWidget (Variables|Default|GetWidget))))
  (bind _output_get (Variables|Default|SetSelectMenu _asselect_menu_fp))
  (Variables|/Game/Blueprints/Menu/WidgetBlueprint/WBP_Select_Menu_FP.WBP_Select_Menu_FP_C|SetUnhoveredColor _output_get (Variables|Default|GetUnhoveredColor))
  (Variables|/Game/Blueprints/Menu/WidgetBlueprint/WBP_Select_Menu_FP.WBP_Select_Menu_FP_C|SetEnumLevelType _output_get (Variables|Default|GetEnumLevelType))
  (Variables|/Game/Blueprints/Menu/WidgetBlueprint/WBP_Select_Menu_FP.WBP_Select_Menu_FP_C|SetHoveredColor _output_get (Variables|Default|GetHoveredColor)))

(event Collision|EventActorBeginOverlap
  (params (OtherActor :type Actor%20Object%20Reference))
  (|CallParentFunction OtherActor) ; This node is disabled and will not be called.\nDrag off pins to build functionality.
)

(event EventTick
  (params (DeltaSeconds :type Float%20%28single-precision%29))
  (|CallParentFunction DeltaSeconds) ; This node is disabled and will not be called.\nDrag off pins to build functionality.
)

(fn ConstructionScript
  (|CallParentFunction))

(fn ToggleWidgetCollision
  (params (Visible :type Boolean))
  (bind _widget (Variables|Default|GetWidget))
  (if Visible
    (Collision|SetCollisionEnabled _widget "QueryOnly")
    (else
      (Collision|SetCollisionEnabled _widget "NoCollision"))))