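; TV actor that shows the drone camera feed and mirrors drone audio while drone controls are enabled.
; It points the drone's scene capture at a render target on game instance enable events, then detaches and clears it on disable.
; MetaSound output watchers track playback of the drone's flying and arm bristle sounds, so the TV's own sounds resume in sync.
; Helper functions forward bristle triggers and stop percent to the TV audio.
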(event Custom|DroneControlsEnabled_Event
  (bind _bristleblastersound (Variables|Default|GetBristleBlasterSound))
  (bind _scenecapturecomponenet2d (Variables|Default|GetSceneCaptureComponenet2D)
    (:then
      (Variables|/Script/Engine.SceneCaptureComponent2D|SetTextureTarget _scenecapturecomponenet2d (Variables|Default|GetTexture%20Target))
      (Development|PrintString "Enabling the render target...")
      (Audio|Parameter|SetFloatParameter (Variables|Default|GetDroneFlyingSound) "StartTime" (stale Custom|PlaybackTime _returnvalue) :!class /Script/AudioExtensions.AudioParameterControllerInterface)
      (Class|AudioParameterControllerInterface|SetTriggerParameter (Variables|Default|GetDroneFlyingSound) "TVSoundStart")
      (if (> (stale Custom|BristlePlaybackTime _returnvalue) 0.0)
        (Audio|Parameter|SetFloatParameter _bristleblastersound "StopPercent" (stale Custom|BristlePlaybackTime _returnvalue) :!class /Script/AudioExtensions.AudioParameterControllerInterface)
        (Class|AudioParameterControllerInterface|SetTriggerParameter _bristleblastersound "Stop")))
    (:else)))

(event Custom|DroneControlsDisabled_Event
  (bind _scenecapturecomponenet2d (Variables|Default|GetSceneCaptureComponenet2D)
    (:then
      (Variables|/Script/Engine.SceneCaptureComponent2D|SetTextureTarget _scenecapturecomponenet2d 0)
      (Rendering|ClearRenderTarget2D (Variables|Default|GetTexture%20Target))
      (Development|PrintString "Disabling the render target...")
      (Class|AudioParameterControllerInterface|SetTriggerParameter (Variables|Default|GetDroneFlyingSound) "TVSoundStop"))
    (:else)))

(event Custom|BristlePlaybackTime
  (params (OutputName :type Name) (Output :type Meta%20Sound%20Output%20Structure%20%28by%20ref%29))
  (bind _returnvalue (Class|MetasoundOutputBlueprintAccess|GetFloat Output)))

(event Custom|PlaybackTime
  (params (OutputName :type Name) (Output :type Meta%20Sound%20Output%20Structure%20%28by%20ref%29))
  (bind _returnvalue (Class|MetasoundOutputBlueprintAccess|GetFloat Output)))

(event EventEndPlay
  (params (EndPlayReason :type EEndPlayReason%20Enum :default "Destroyed"))
  (bind _asbp_wind_turbine_game_instance (Utilities|Casting|CastToBP_WindTurbine_GameInstance (Game|GetGameInstance)))
  (EventDispatchers|UnbindallEventsfromDroneControlsDisabled _asbp_wind_turbine_game_instance)
  (EventDispatchers|UnbindallEventsfromDroneControlsEnabled _asbp_wind_turbine_game_instance))

(event EventBeginPlay
  (bind _returnvalue (WorldSubsystems|GetMetaSoundOutputSubsystem))
  (bind _returnvalue_2 (Actor|GetActorOfClass "/Game/Blueprints/Drone/BP_Drone.BP_Drone_C"))
  (bind _output_get (Variables|Default|SetDroneRef _returnvalue_2))
  (bind _output_get_2 (Variables|Default|SetSceneCaptureComponenet2D (Variables|/Game/Blueprints/Drone/BP_Drone.BP_Drone_C|GetDroneCamera _output_get)))
  (Variables|/Script/Engine.SceneCaptureComponent2D|SetTextureTarget _output_get_2 (Variables|Default|GetTexture%20Target))
  (bind _asbp_wind_turbine_game_instance (Utilities|Casting|CastToBP_WindTurbine_GameInstance (Game|GetGameInstance)))
  (EventDispatchers|AssignDroneControlsEnabled _asbp_wind_turbine_game_instance (delegate Custom|DroneControlsEnabled_Event))
  (EventDispatchers|AssignDroneControlsDisabled _asbp_wind_turbine_game_instance (delegate Custom|DroneControlsDisabled_Event))
  (MetaSoundOutput|WatchOutput _returnvalue (Variables|/Game/Blueprints/Drone/BP_Drone.BP_Drone_C|GetDroneFlyingSound (Variables|Default|GetDroneRef)) "CurrentPlaybackTime" (delegate Custom|PlaybackTime) "None" "None" :!class /Script/MetasoundEngine.MetaSoundOutputSubsystem)
  (CallFunction|DroneControlsDisabledEvent)
  (bind _asbp_drone_arm (Utilities|Casting|CastToBP_DroneArm (Variables|/Script/Engine.ChildActorComponent|GetChildActor (Variables|/Game/Blueprints/Drone/BP_Drone.BP_Drone_C|GetBP_RobotArm (Variables|Default|GetDroneRef)))))
  (MetaSoundOutput|WatchOutput _returnvalue (Variables|/Game/Blueprints/Drone/DroneArm/BP_DroneArm.BP_DroneArm_C|GetBristleSound _asbp_drone_arm) "CurrentPlaybackPercent" (delegate Custom|BristlePlaybackTime) "None" "None" :!class /Script/MetasoundEngine.MetaSoundOutputSubsystem)
  (Audio|Parameter|SetFloatParameter (Variables|Default|GetBristleBlasterSound) "StopPercent" 1.0 :!class /Script/AudioExtensions.AudioParameterControllerInterface))

(fn ConstructionScript)

(fn SetBristleSounds
  (params (TriggerName :type Name))
  (Class|AudioParameterControllerInterface|SetTriggerParameter (Variables|Default|GetBristleBlasterSound) TriggerName))

(fn SetStopPercent
  (params (Percent :type Float%20%28double-precision%29))
  (Audio|Parameter|SetFloatParameter (Variables|Default|GetBristleBlasterSound) "StopPercent" Percent :!class /Script/Engine.AudioComponent))