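; TV actor that shows the live camera feed from the first BP_Drone in the level while drone controls are enabled.
; On BeginPlay it routes the drone's scene capture into a render target, applies the screen material to its cube and binds to the game instance's control events.
; Those events attach the render target, or detach it and clear it to black.
; EndPlay unbinds all listeners from both dispatchers.
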(event Custom|DroneControlsEnabled_Event
  (bind _scenecapturecomponenet2d (Variables|Default|GetSceneCaptureComponenet2D)
    (:then
      (Variables|/Script/Engine.SceneCaptureComponent2D|SetTextureTarget _scenecapturecomponenet2d (Variables|Default|GetTexture%20Target))
      (Development|PrintString "Enabling the render target..."))
    (:else)))

(event Custom|DroneControlsDisabled_Event
  (bind _scenecapturecomponenet2d (Variables|Default|GetSceneCaptureComponenet2D)
    (:then
      (Variables|/Script/Engine.SceneCaptureComponent2D|SetTextureTarget _scenecapturecomponenet2d 0)
      (Rendering|ClearRenderTarget2D (Variables|Default|GetTexture%20Target))
      (Development|PrintString "Disabling the render target..."))
    (:else)))

(event EventEndPlay
  (params (EndPlayReason :type EEndPlayReason%20Enum :default "Destroyed"))
  (bind _ascustom_game_instance (Utilities|Casting|CastToBP_CustomGameInstance (Game|GetGameInstance)))
  (EventDispatchers|UnbindallEventsfromDroneControlsDisabled _ascustom_game_instance)
  (EventDispatchers|UnbindallEventsfromDroneControlsEnabled _ascustom_game_instance))

(event EventBeginPlay
  (bind _outactors (Actor|GetAllActorsOfClass "/Game/Blueprints/Drone/BP_Drone.BP_Drone_C"))
  (bind _output_get (Variables|Default|SetSceneCaptureComponenet2D (Variables|/Game/Blueprints/Drone/BP_Drone.BP_Drone_C|GetDroneCamera (Utilities|Array|Get(acopy) _outactors))))
  (Variables|/Script/Engine.SceneCaptureComponent2D|SetTextureTarget _output_get (Variables|Default|GetTexture%20Target))
  (Rendering|Material|SetMaterial (Variables|Default|GetCube) 0 (Variables|Default|GetMaterial))
  (bind _ascustom_game_instance (Utilities|Casting|CastToBP_CustomGameInstance (Game|GetGameInstance)))
  (EventDispatchers|AssignDroneControlsEnabled _ascustom_game_instance (delegate Custom|DroneControlsEnabled_Event))
  (EventDispatchers|AssignDroneControlsDisabled _ascustom_game_instance (delegate Custom|DroneControlsDisabled_Event))
  (CallFunction|DroneControlsDisabledEvent))

(fn ConstructionScript)