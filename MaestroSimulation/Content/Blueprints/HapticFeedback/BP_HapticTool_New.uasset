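; Haptic bristle blaster tool, a grippable powered tool with two hand sockets, a paint component and MetaSound audio.
; Activation, socket haptics and scale queries delegate to BPBristleComponent, whose rotation and button values drive the animation Blueprint each tick.
; A watched MetaSound "StartFinished" output sets the running state, then collision polling switches between running and colliding sounds.
; Active scale feeds the sound's stop parameter, and paint completion triggers a win sound.
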(event Custom|CustomEvent
  (params (OutputName :type Name) (Output :type Meta%20Sound%20Output%20Structure%20%28by%20ref%29))
  (Variables|Default|SetCurrentState "NewEnumerator1"))

(event Custom|OnPaintComplete_Event
  (Class|AudioParameterControllerInterface|SetTriggerParameter (Variables|Default|GetSound) "Win"))

(event EventBeginPlay
  (MetaSoundOutput|WatchOutput (WorldSubsystems|GetMetaSoundOutputSubsystem) (Variables|Default|GetSound) "StartFinished" (delegate Custom|CustomEvent) "None" "None" :!class /Script/MetasoundEngine.MetaSoundOutputSubsystem)
  (EventDispatchers|AssignOnPaintComplete (Variables|Default|GetBP_PaintComponent) (delegate Custom|OnPaintComplete_Event)))

(event EventTick
  (params (DeltaSeconds :type Float%20%28single-precision%29))
  (Utilities|FlowControl|Sequence
    (:then_0
      (Utilities|FlowControl|DoOnce false
        (:Completed
          (CallFunction|Setup))))
    (:then_1
      (CallFunction|UpdateAnimationValues))))

(fn ConstructionScript)

(fn Setup
  (Default|Setup (Variables|Default|GetBP_BristleComponent) (Variables|Default|GetInnerStaticMesh) (Variables|Default|GetOuterStaticMesh) (Variables|Default|GetLowerHandSocket) (Variables|Default|GetUpperHandSocket) (Variables|Default|GetBP_PaintComponent) false (Variables|Default|GetSound))
  ;[0.15 0.15 0.15 0.5] Get Animation Blueprint of Skeletal Mesh
  (bind _asabp_bristle_blaster (Utilities|Casting|CastToABP_Bristle_Blaster (Components|SkeletalMesh|GetAnimInstance (Variables|Default|GetGrippableSkeletalMesh))))
  (Variables|Default|SetBristleBlasterAnim _asabp_bristle_blaster))

(fn SetActivenessHandSocket
  (params (HandSocket :type String) (State :type Boolean))
  (Default|SetActivenessHandSocket (Variables|Default|GetBP_BristleComponent) HandSocket State))

(fn GetSocketHapticMultiplier
  (params (HandSocket :type String))
  (bind _multiplier (Default|GetSocketHapticMultiplier (Variables|Default|GetBP_BristleComponent) HandSocket))
  (return _multiplier))

(fn GetCollisionScale
  (if (Utilities|Enum|NotEqual(Enum) (Variables|Default|GetCurrentState) "NewEnumerator0")
    (bind (_scale _result) (Default|GetCollisionScale (Variables|Default|GetBP_BristleComponent)))
    (if (Math|Boolean|ANDBoolean _result (Utilities|Enum|Equal(Enum) (Variables|Default|GetCurrentState) "NewEnumerator1") (Utilities|Enum|NotEqual(Enum) (Variables|Default|GetCurrentState) "NewEnumerator2"))
      (Variables|Default|SetCurrentState "NewEnumerator2")
      (Class|AudioParameterControllerInterface|SetTriggerParameter (Variables|Default|GetSound) "Collision")
      (elif (and (not _result) (Utilities|Enum|Equal(Enum) (Variables|Default|GetCurrentState) "NewEnumerator2"))
        (Variables|Default|SetCurrentState "NewEnumerator1")
        (Class|AudioParameterControllerInterface|SetTriggerParameter (Variables|Default|GetSound) "Running")))
    (return _scale _result)
    (else
      (return 0.0 false))))

(fn Activate
  (Default|Turnon (Variables|Default|GetBP_BristleComponent)))

(fn Deactivate
  (Default|TurnOff (Variables|Default|GetBP_BristleComponent)))

(fn GetActiveScale
  (bind (_activescale _adjactivescale) (Default|GetActiveScale (Variables|Default|GetBP_BristleComponent)))
  (Audio|Parameter|SetFloatParameter (Variables|Default|GetSound) "StopPercent" (- 1.0 _activescale) :!class /Script/Engine.AudioComponent)
  (return _activescale _adjactivescale))

(fn UpdateAnimationValues
  (bind _bp_bristlecomponent (Variables|Default|GetBP_BristleComponent))
  (bind _bristleblasteranim (Variables|Default|GetBristleBlasterAnim))
  (Utilities|IsValid _bristleblasteranim
    (:Is%20Valid
      (Variables|/Game/BristleBlaster/New/ABP_Bristle_Blaster.ABP_Bristle_Blaster_C|SetBlasterRotation _bristleblasteranim (Variables|/Game/Blueprints/HapticFeedback/BP_BristleComponent.BP_BristleComponent_C|GetCurrentBristleRotation _bp_bristlecomponent))
      (Variables|/Game/BristleBlaster/New/ABP_Bristle_Blaster.ABP_Bristle_Blaster_C|SetButtonRotation _bristleblasteranim (Variables|/Game/Blueprints/HapticFeedback/BP_BristleComponent.BP_BristleComponent_C|GetButtonScale _bp_bristlecomponent)))))