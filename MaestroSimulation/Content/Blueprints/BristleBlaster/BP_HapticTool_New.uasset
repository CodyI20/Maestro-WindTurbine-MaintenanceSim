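; VR grippable Bristle Blaster tool that hands its activation, hand-socket haptics and scale queries to BPBristleComponent.
; The first Tick runs Setup once, passing the collision meshes, hand sockets and paint component to that component and caching the mesh's anim instance.
; Every Tick copies bristle rotation and button scale into ABP_BristleBlaster.
; BeginPlay starts BristleBlaster playback with its IsRunning parameter set true.
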(event EventTick
  (params (DeltaSeconds :type Float%20%28single-precision%29))
  (Utilities|FlowControl|Sequence
    (:then_0
      (Utilities|FlowControl|DoOnce false
        (:Completed
          (CallFunction|Setup))))
    (:then_1
      (CallFunction|UpdateAnimationValues))))

(event EventBeginPlay
  (bind _bristleblaster (Variables|Default|GetBristleBlaster))
  (Effects|Components|ParticleSystem|SetBoolParameter _bristleblaster "IsRunning" true)
  (Audio|Components|Audio|Play _bristleblaster 0.0))

(fn ConstructionScript)

(fn Setup
  (Default|Setup (Variables|Default|GetBP_BristleComponent) (Variables|Default|GetInnerStaticMesh) (Variables|Default|GetOuterStaticMesh) (Variables|Default|GetLowerHandSocket) (Variables|Default|GetUpperHandSocket) (Variables|Default|GetBP_PaintComponent) false)
  ;[0.15 0.15 0.15 0.5] Get Animation Blueprint of Skeletal Mesh
  (bind _asabp_bristle_blaster (Utilities|Casting|CastToABP_BristleBlaster (Components|SkeletalMesh|GetAnimInstance (Variables|Default|GetGrippableSkeletalMesh))))
  (Variables|Default|SetBristleBlasterAnim _asabp_bristle_blaster))

(fn SetActivenessHandSocket
  (params (HandSocket :type String) (State :type Boolean))
  (Default|SetActivenessHandSocket (Variables|Default|GetBP_BristleComponent) HandSocket State))

(fn GetSocketHapticMultiplier
  (params (HandSocket :type String))
  (bind _multiplier (Default|GetSocketHapticMultiplier (Variables|Default|GetBP_BristleComponent) HandSocket))
  (return _multiplier))

(fn GetCollisionScale
  (bind (_scale _result) (Default|GetCollisionScale (Variables|Default|GetBP_BristleComponent)))
  (return _scale _result))

(fn Activate
  (Variables|/Game/Blueprints/BristleBlaster/BP_BristleComponent.BP_BristleComponent_C|SetIsActivated (Variables|Default|GetBP_BristleComponent) true))

(fn Deactivate
  (Variables|/Game/Blueprints/BristleBlaster/BP_BristleComponent.BP_BristleComponent_C|SetIsActivated (Variables|Default|GetBP_BristleComponent) false))

(fn GetActiveScale
  (bind (_activescale _adjactivescale) (Default|GetActiveScale (Variables|Default|GetBP_BristleComponent)))
  (return _activescale _adjactivescale))

(fn UpdateAnimationValues
  (bind _bp_bristlecomponent (Variables|Default|GetBP_BristleComponent))
  (bind _bristleblasteranim (Variables|Default|GetBristleBlasterAnim))
  (Utilities|IsValid _bristleblasteranim
    (:Is%20Valid
      (Variables|/Game/Models/BristleBlaster/ABP_BristleBlaster.ABP_BristleBlaster_C|SetBlasterRotation _bristleblasteranim (Variables|/Game/Blueprints/BristleBlaster/BP_BristleComponent.BP_BristleComponent_C|GetCurrentBristleRotation _bp_bristlecomponent))
      (Variables|/Game/Models/BristleBlaster/ABP_BristleBlaster.ABP_BristleBlaster_C|SetButtonRotation _bristleblasteranim (Variables|/Game/Blueprints/BristleBlaster/BP_BristleComponent.BP_BristleComponent_C|GetButtonScale _bp_bristlecomponent)))))