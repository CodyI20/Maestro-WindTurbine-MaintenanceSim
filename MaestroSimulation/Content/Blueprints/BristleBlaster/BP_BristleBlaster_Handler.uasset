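; Handles the state of a VR Bristle Blaster tool (or drone variant): activation, bristle contact, haptic scaling and sound.
; Tick ramps activation scale and bristle rotation, with MetaSound's startup output switching it to running.
; A fan of line traces between measured bristle radii drives painting via PaintComponent and returns contact strength.
; State changes trigger MetaSound cues mirrored to a TV actor, while hand sockets can be disabled and carry haptic multipliers.
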(event Custom|SubscribeEvent
  (MetaSoundOutput|WatchOutput (WorldSubsystems|GetMetaSoundOutputSubsystem) (Variables|Default|GetSound) "StartFinished" (delegate Custom|StartupFinished) "None" "None" :!class /Script/MetasoundEngine.MetaSoundOutputSubsystem))

(event Custom|StartupFinished
  (params (OutputName :type Name) (Output :type Meta%20Sound%20Output%20Structure%20%28by%20ref%29))
  (Variables|Default|SetCurrentState "NewEnumerator1"))

(event EventTick
  (params (DeltaSeconds :type Float%20%28single-precision%29))
  (Utilities|FlowControl|Sequence
    (:then_0
      (Utilities|FlowControl|DoOnce false
        (:Completed
          (CallFunction|Initialize))))
    (:then_1
      (Activation|UpdateActivation)
      (CallFunction|UpdateAnimationValues))))

(fn Setup
  (params (InnerSphereCol :type Static%20Mesh%20Component%20Object%20Reference) (OuterSphereCol :type Static%20Mesh%20Component%20Object%20Reference) (LowerHandSocket :type Hand%20Socket%20Base%20Object%20Reference) (UpperHandSocket :type Hand%20Socket%20Base%20Object%20Reference) (PaintComponent :type BP%20Paint%20Component%20Object%20Reference) (IsDrone :type Boolean) (Sound :type Audio%20Component%20Object%20Reference))
  (Variables|Default|SetInnerSphereMesh InnerSphereCol)
  (Variables|Default|SetOuterSphereMesh OuterSphereCol)
  (Variables|Default|SetLowerHandSocket LowerHandSocket)
  (Variables|Default|SetUpperHandSocket UpperHandSocket)
  (Variables|Default|SetPaintComponent PaintComponent)
  (Variables|Default|SetIsDrone IsDrone)
  (Variables|Default|SetSound Sound)
  (CallFunction|SubscribeEvent))

(fn Turnon
  (Variables|Activation|SetIsActivated true)
  (Variables|Default|SetCurrentState "NewEnumerator0")
  (Class|AudioParameterControllerInterface|SetTriggerParameter (Variables|Default|GetSound) "Start")
  (bind _tvinstance (Variables|Components|GetTVInstance)
    (:then
      (Default|SetBristleSounds _tvinstance "Start"))
    (:else)))

(fn TurnOff
  (Variables|Activation|SetIsActivated false)
  (Variables|Default|SetCurrentState "NewEnumerator3")
  (Class|AudioParameterControllerInterface|SetTriggerParameter (Variables|Default|GetSound) "Stop")
  (bind _tvinstance (Variables|Components|GetTVInstance)
    (:then
      (Default|SetBristleSounds _tvinstance "Stop"))
    (:else)))

(fn UpdateActivation
  (bind _returnvalue (Utilities|Time|GetWorldDeltaSeconds))
  (bind _returnvalue_2 (Utilities|Time|GetWorldDeltaSeconds))
  (bind _increasespeedbutton (Variables|Activation|GetIncreaseSpeedButton))
  (bind _minhapticactivation (Variables|Activation|GetMinHapticActivation))
  (bind _maxhapticactivation (Variables|Activation|GetMaxHapticActivation))
  (bind _increasespeedactivescale (Variables|Activation|GetIncreaseSpeedActiveScale))
  (bind _returnvalue_3 (* _returnvalue_2 _increasespeedbutton))
  (bind _returnvalue_4 (* _returnvalue _increasespeedactivescale))
  ;[0.15 0.15 0.15 0.5] Update current active scale
  (if (Variables|Activation|GetIsActivated)
    (if (< (Variables|Activation|GetActiveScale) 1.0)
      (Variables|Activation|SetActiveScale (Math|Float|Clamp(Float) (+ (Variables|Activation|GetActiveScale) _returnvalue_4) _minhapticactivation _maxhapticactivation))
      (Variables|Activation|SetButtonScale (Math|Float|Clamp(Float) (+ (Variables|Activation|GetButtonScale) _returnvalue_3) 0.0 2.5)))
    (else
      (Variables|Activation|SetActiveScale (Math|Float|Clamp(Float) (- (Variables|Activation|GetActiveScale) _returnvalue_4) _minhapticactivation _maxhapticactivation))
      (Variables|Activation|SetButtonScale (Math|Float|Clamp(Float) (- (Variables|Activation|GetButtonScale) _returnvalue_3) 0.0 2.5)))))

(fn Initialize
  (bind _outerspheremesh (Variables|Default|GetOuterSphereMesh))
  (bind _returnvalue (Transformation|GetWorldLocation _outerspheremesh))
  (Utilities|FlowControl|Sequence
    (:then_0
      ;[0.15 0.15 0.15 0.5] Get hands to ignore during raycast, and set player controller reference for repeated use
      (bind _asbp_vrcharacter (Utilities|Casting|CastToBP_VRCharacter (Game|GetPlayerCharacter 0))
        (:then
          (bind _output_get (Variables|Default|SetIgnoreArray (Utilities|Array|MakeArray (Variables|/Game/VRE/Core/Character/BP_VRCharacter.BP_VRCharacter_C|GetGraspingHandLeft _asbp_vrcharacter) (Variables|/Game/VRE/Core/Character/BP_VRCharacter.BP_VRCharacter_C|GetGraspingHandRight _asbp_vrcharacter) _asbp_vrcharacter))))
        (:CastFailed
          _))
      (Variables|Default|SetPlayerController (Game|GetPlayerController 0))
      ;[0.15 0.15 0.15 0.5] Add other actors to be ignored
      (bind _outactors (Actor|GetAllActorswithTag "IgnoreBristleRay"))
      (for _array_element _outactors
        (Utilities|Array|Add _output_get _array_element)
        ;[0.15 0.15 0.15 0.5] Get TV reference to play sounds there too
        (bind _returnvalue_2 (Actor|GetActorOfClass "/Game/Cody/TV/TV.TV_C"))
        (Variables|Components|SetTVInstance _returnvalue_2)))
    (:then_1
      ;[0.15 0.15 0.15 0.5] Calculate bristle radius (start distance from center to inner collider), to be used for mapping for scale value
      (bind _outhits (Class|KismetSystemLibrary|LineTraceMultiforObjects (+ _returnvalue (* (Math|Vector|GetUpVector _outerspheremesh) 1e+02)) _returnvalue (Utilities|Array|MakeArray "ObjectTypeQuery1" "ObjectTypeQuery2") true 0 "None" false))
      (for _array_element_2 _outhits
        (if (== (.HitComponent (Collision|BreakHitResult _array_element_2)) (Variables|Default|GetInnerSphereMesh))
          (bind _output_get_2 (LocalVariables|SetInnerRadius (- (Transformation|GetWorldLocation (Variables|Default|GetOuterSphereMesh)) (.ImpactPoint (Collision|BreakHitResult _array_element_2)))))
          (Variables|Default|SetMinBristleRadius (Math|Vector|VectorLength _output_get_2))
          (elif (== (.HitComponent (Collision|BreakHitResult _array_element_2)) (Variables|Default|GetOuterSphereMesh))
            (bind _output_get_3 (LocalVariables|SetOuterRadius (- (Transformation|GetWorldLocation (Variables|Default|GetOuterSphereMesh)) (.ImpactPoint (Collision|BreakHitResult _array_element_2)))))
            (Variables|Default|SetMaxBristleRadius (Math|Vector|VectorLength (- (LocalVariables|GetInnerRadius) _output_get_3))))))
      (Rendering|SetVisibility (Variables|Default|GetInnerSphereMesh) false true))
    (:then_2
      ;[0.15 0.15 0.15 0.5] Create library to identify hand socket in use
      (if (not (Variables|Default|GetIsDrone))
        (for _array_element_3 (Utilities|Array|MakeArray (Variables|Default|GetLowerHandSocket) (Variables|Default|GetUpperHandSocket))
          (Utilities|Map|Add (Variables|Default|GetHandSockets) (Utilities|GetObjectName _array_element_3) _array_element_3))
        (else
          (return))))
    (:then_3
      ;[0.15 0.15 0.15 0.5] Note which sockets to reduce haptic feedback to
      (Utilities|FlowControl|Sequence
        (:then_0
          (Utilities|Map|Add (Variables|Default|GetSocketHapticMultiplier) (Utilities|GetObjectName (Variables|Default|GetLowerHandSocket)) (- 1.0 (Variables|Default|GetHapticMultiplierReduction))))
        (:then_1
          (Utilities|Map|Add (Variables|Default|GetSocketHapticMultiplier) (Utilities|GetObjectName (Variables|Default|GetUpperHandSocket)) 1.0))))))

(fn SetActivenessHandSocket
  (params (HandSocket :type String) (State :type Boolean))
  (bind _handsockets (Variables|Default|GetHandSockets))
  (bind (_value _returnvalue) (Utilities|Map|Find _handsockets HandSocket))
  (if (not (Variables|Default|GetIsDrone))
    ;[0.15 0.15 0.15 0.5] Disables / Enables the spots on the instrument, to which the hands attach
    (if _returnvalue
      (if State
        (Variables|/Script/VRExpansionPlugin.HandSocketComponent|SetbDisabled _value false)
        (else
          (Variables|/Script/VRExpansionPlugin.HandSocketComponent|SetbDisabled _value true))))))

(fn GetSocketHapticMultiplier
  (params (HandSocket :type String))
  (if (not (Variables|Default|GetIsDrone))
    ;[0.15 0.15 0.15 0.5] Different spots on the instrument apply different scales of haptics
    (return (.Value (Utilities|Map|Find (Variables|Default|GetSocketHapticMultiplier) HandSocket)))
    (else
      (return 1.0))))

(fn GetCollisionScale
  (bind _outerspheremesh (Variables|Default|GetOuterSphereMesh))
  (bind _outerspheremesh_2 (Variables|Default|GetOuterSphereMesh))
  (bind _returnvalue (Transformation|GetWorldLocation _outerspheremesh_2))
  (if (and (Variables|Activation|GetIsActivated) (Utilities|Enum|NotEqual(Enum) (Variables|Default|GetCurrentState) "NewEnumerator0"))
    (LocalVariables|SetAnglePerRay (/ 220 (Variables|Default|GetRayCount)))
    ;[0.15 0.15 0.15 0.5] Perform raycasts around the y axis, spreading them based on rayCount
    (for _index (range 0 (- (Variables|Default|GetRayCount) 1))
      (LocalVariables|SetRayStart (+ _returnvalue (* (Math|Vector|RotateVectorAroundAxis (Math|Vector|GetUpVector _outerspheremesh) (* _index (LocalVariables|GetAnglePerRay)) (Math|Vector|GetRightVector _outerspheremesh)) (- (Variables|Default|GetMinBristleRadius) 1.5))))
      (LocalVariables|SetRayEnd (+ _returnvalue (* (Math|Vector|RotateVectorAroundAxis (Math|Vector|GetUpVector _outerspheremesh) (* _index (LocalVariables|GetAnglePerRay)) (Math|Vector|GetRightVector _outerspheremesh)) (Variables|Default|GetMaxBristleRadius))))
      ;[0.15 0.15 0.15 0.5] Apply painting onto Render Target Canvas, using the collision surface normal
      (bind (_outhit _returnvalue_2) (Collision|LineTraceByChannel (LocalVariables|GetRayStart) (LocalVariables|GetRayEnd) "TraceTypeQuery1" true (Variables|Default|GetIgnoreArray) "None"))
      (if _returnvalue_2
        (LocalVariables|SetImpactPoint (.ImpactPoint (Collision|BreakHitResult _outhit)))
        (LocalVariables|SetImpactNormal (.ImpactNormal (Collision|BreakHitResult _outhit)))
        (if (> (Math|Float|MapRangeClamped (.Distance (Collision|BreakHitResult _outhit)) (Math|Vector|VectorLength (- (LocalVariables|GetRayEnd) (LocalVariables|GetRayStart))) 0.0 (Variables|Activation|GetActiveScaleBoundary) 1.0) (LocalVariables|GetHighestScale))
          (bind _output_get (LocalVariables|SetHighestScale (Math|Float|MapRangeClamped (.Distance (Collision|BreakHitResult _outhit)) (Math|Vector|VectorLength (- (LocalVariables|GetRayEnd) (LocalVariables|GetRayStart))) 0.0 (Variables|Activation|GetActiveScaleBoundary) 1.0))))
        (bind _result (Default|UpdatePainting (Variables|Default|GetPaintComponent) _output_get _outhit))
        (LocalVariables|SetPaintResult _result)))
    ;[0.15 0.15 0.15 0.5] Update state and return scale
    (if (Math|Boolean|ANDBoolean (LocalVariables|GetPaintResult) (Utilities|Enum|Equal(Enum) (Variables|Default|GetCurrentState) "NewEnumerator1") (Utilities|Enum|NotEqual(Enum) (Variables|Default|GetCurrentState) "NewEnumerator2"))
      (Variables|Default|SetCurrentState "NewEnumerator2")
      (Class|AudioParameterControllerInterface|SetTriggerParameter (Variables|Default|GetSound) "Collision")
      (bind _tvinstance (Variables|Components|GetTVInstance)
        (:then
          (Default|SetBristleSounds _tvinstance "Collision"))
        (:else
          _))
      (elif (and (not (LocalVariables|GetPaintResult)) (Utilities|Enum|Equal(Enum) (Variables|Default|GetCurrentState) "NewEnumerator2"))
        (Variables|Default|SetCurrentState "NewEnumerator1")
        (Class|AudioParameterControllerInterface|SetTriggerParameter (Variables|Default|GetSound) "Running")
        (bind _tvinstance_2 (Variables|Components|GetTVInstance)
          (:then
            (Default|SetBristleSounds _tvinstance_2 "Running"))
          (:else
            _))))
    (return (* (LocalVariables|GetHighestScale) 1e+02) (LocalVariables|GetPaintResult))
    (else
      (return 0.0 false))))

(fn GetActiveScale
  (bind _activescale (Variables|Activation|GetActiveScale))
  (bind _returnvalue (- 1.0 _activescale))
  (Audio|Parameter|SetFloatParameter (Variables|Default|GetSound) "StopPercent" _returnvalue :!class /Script/Engine.AudioComponent)
  (bind _tvinstance (Variables|Components|GetTVInstance)
    (:then
      (Default|SetStopPercent _tvinstance _returnvalue))
    (:else
      _))
  (return _activescale (* _activescale (Variables|Activation|GetActiveScaleBoundary))))

(fn UpdateAnimationValues
  (Variables|Activation|SetCurrentBristleRotation (Math|Float|%(Float) (+ (Variables|Activation|GetCurrentBristleRotation) (* (* (* (Variables|Activation|GetBristleMaxSpeed) 1.0) (Variables|Activation|GetActiveScale)) (Utilities|Time|GetWorldDeltaSeconds))) 3.6e+02)))

(fn PlayWin
  (Class|AudioParameterControllerInterface|SetTriggerParameter (Variables|Default|GetSound) "Win")
  (bind _tvinstance (Variables|Components|GetTVInstance)
    (:then
      (Default|SetBristleSounds _tvinstance "Win"))
    (:else)))