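; BP_BristleBlaster is a grippable, hand-held bristle blaster tool with on/off control, hand sockets and haptics.
; A first-tick setup wires collision meshes, hand sockets, paint component and sound into BPBristleComponent, which handles activation and per-socket haptic multipliers.
; Every tick it copies bristle rotation and button values from that component into the animation blueprint.
; When the paint component reports completion, the bristle component plays a win response.
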(event Custom|OnPaintComplete_Event
  (Default|PlayWin (Variables|Default|GetBP_BristleComponent)))

(event EventBeginPlay
  (EventDispatchers|AssignOnPaintComplete (Variables|Default|GetBP_PaintComponent) (delegate Custom|OnPaintComplete_Event)))

(event EventTick
  (params (DeltaSeconds :type Float%20%28single-precision%29))
  (Utilities|FlowControl|Sequence
    (:then_0
      (Utilities|FlowControl|DoOnce false
        (:Completed
          (CallFunction|Setup))))
    (:then_1
      (CallFunction|UpdateAnimationValues))))

(fn ConstructionScript)

(fn Setup
  (Default|Setup (Variables|Default|GetBP_BristleComponent) (Variables|Default|GetInnerStaticMesh) (Variables|Default|GetOuterStaticMesh) (Variables|Default|GetLowerHandSocket) (Variables|Default|GetUpperHandSocket) (Variables|Default|GetBP_PaintComponent) false (Variables|Default|GetSound))
  ;[0.15 0.15 0.15 0.5] Get Animation Blueprint of Skeletal Mesh
  (bind _asabp_bristle_blaster (Utilities|Casting|CastToABP_BristleBlaster (Components|SkeletalMesh|GetAnimInstance (Variables|Default|GetGrippableSkeletalMesh))))
  (Variables|Default|SetBristleBlasterAnim _asabp_bristle_blaster))

(fn GetSocketHapticMultiplier
  (params (HandSocket :type String))
  (bind _multiplier (Default|GetSocketHapticMultiplier (Variables|Default|GetBP_BristleComponent) HandSocket))
  (return _multiplier))

(fn Activate
  (Default|Turnon (Variables|Default|GetBP_BristleComponent)))

(fn Deactivate
  (Default|TurnOff (Variables|Default|GetBP_BristleComponent)))

(fn UpdateAnimationValues
  (bind _bp_bristlecomponent (Variables|Default|GetBP_BristleComponent))
  (bind _bristleblasteranim (Variables|Default|GetBristleBlasterAnim))
  (Utilities|IsValid _bristleblasteranim
    (:Is%20Valid
      (Variables|/Game/Models/BristleBlaster/ABP_BristleBlaster.ABP_BristleBlaster_C|SetBlasterRotation _bristleblasteranim (Variables|/Game/Blueprints/BristleBlaster/BP_BristleBlaster_Handler.BP_BristleBlaster_Handler_C|GetCurrentBristleRotation _bp_bristlecomponent))
      (Variables|/Game/Models/BristleBlaster/ABP_BristleBlaster.ABP_BristleBlaster_C|SetButtonRotation _bristleblasteranim (Variables|/Game/Blueprints/BristleBlaster/BP_BristleBlaster_Handler.BP_BristleBlaster_Handler_C|GetButtonScale _bp_bristlecomponent)))))