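; Offshore wind turbine actor whose patch mesh gets an outline effect through an outline handler component.
; BeginPlay sets up the handler with the mesh, a sphere collider and an outline material.
; The first Tick caches the mesh's dynamic material, then each Tick polls its DeactivateOutline scalar.
; Once that value reaches one, the actor deactivates the handler and marks the outline finished.
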(event EventBeginPlay
  (Default|Setup (Variables|Default|GetBP_OutlineHandler) (Variables|Default|GetWindTurbine_OffShore_Patch) (Variables|Default|GetSphere) "/Game/Materials/Outline/old/MI_Outline_1.MI_Outline_1" 2.0))

(event EventTick
  (params (DeltaSeconds :type Float%20%28single-precision%29))
  (Utilities|FlowControl|Sequence
    (:then_0
      (Utilities|FlowControl|DoOnce false
        (:Completed
          (bind _asmaterial_instance_dynamic (Utilities|Casting|CastToMaterialInstanceDynamic (Rendering|Material|GetMaterial (Variables|Default|GetWindTurbine_OffShore_Patch) 0)))
          (Variables|Default|SetPatchDynamicMaterial _asmaterial_instance_dynamic))))
    (:then_1
      (CallFunction|CheckOutlineState))))

(fn ConstructionScript)

(fn CheckOutlineState
  (if (not (Variables|Default|GetOutlineFinished))
    (bind _patchdynamicmaterial (Variables|Default|GetPatchDynamicMaterial)
      (:then
        (bind _returnvalue (Rendering|Material|GetScalarParameterValue _patchdynamicmaterial "DeactivateOutline" :!class /Script/Engine.MaterialInstanceDynamic))
        (if (>= _returnvalue 1.0)
          (Default|DeactivateComponent (Variables|Default|GetBP_OutlineHandler))
          (Variables|Default|SetOutlineFinished true)))
      (:else))))