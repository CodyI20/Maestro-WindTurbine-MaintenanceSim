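; BP_SoundTransitioner computes a sound scale from the VR player character's height between two markers, Lowest and Highest.
; One tick after BeginPlay, Setup caches both markers' world Z values and the player's BP_VRCharacter.
; Each Tick maps the character's Z, clamped to that range, from LowestSoundValue up to full scale in SoundsScale.
; Nothing in this graph applies the value to audio.
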(event EventBeginPlay
  (Utilities|FlowControl|DelayUntilNextTick)
  (CallFunction|Setup))

(event EventTick
  (params (DeltaSeconds :type Float%20%28single-precision%29))
  (CallFunction|UpdateSoundScale))

(fn ConstructionScript)

(fn Setup
  (Variables|Default|SetLowestHeight (.z (Transformation|GetWorldLocation (Variables|Default|GetLowest))))
  (Variables|Default|SetGreatestHeight (.z (Transformation|GetWorldLocation (Variables|Default|GetHighest))))
  (bind _asbp_vrcharacter (Utilities|Casting|CastToBP_VRCharacter (Game|Player|GetPlayerPawn 0)))
  (Variables|Default|SetCharacter _asbp_vrcharacter))

(fn UpdateSoundScale
  (Utilities|IsValid (Variables|Default|GetCharacter)
    (:Is%20Valid
      (Variables|Default|SetSoundsScale (Math|Float|MapRangeClamped (.z (Transformation|GetActorLocation (Variables|Default|GetCharacter))) (Variables|Default|GetLowestHeight) (Variables|Default|GetGreatestHeight) (Variables|Default|GetLowestSoundValue) 1.0)))))