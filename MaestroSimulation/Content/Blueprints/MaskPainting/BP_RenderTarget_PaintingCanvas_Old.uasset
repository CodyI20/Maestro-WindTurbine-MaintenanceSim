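; Paintable canvas actor that lets the BP_HapticTool paint onto its static mesh through a render target.
; Setup clears the target, creates a dynamic brush material reading it, and makes a matching copy.
; Each tick copies the duplicate back into the main target, then line-traces along the tool's up vector.
; Hits pass collision UVs to the brush, which draws into the copy, accumulating strokes through this ping-pong.
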(event EventBeginPlay
  (CallFunction|Setup))

(event EventTick
  (params (DeltaSeconds :type Float%20%28single-precision%29))
  (bind _drawtool (Variables|Settings|GetDrawTool))
  (bind _returnvalue (Transformation|GetActorLocation _drawtool))
  ;[0.15 0.15 0.15 0.5] Update the copy of the material instance
  (Utilities|FlowControl|Sequence
    (:then_0
      (bind (_canvas _size _context) (Rendering|BeginDrawCanvastoRenderTarget (Variables|Settings|GetPaintingRenderTarget)))
      (Canvas|DrawTexture :self _canvas :RenderTexture (Variables|State|GetPaintingRenderTargetCopy) :ScreenSize _size :CoordinateSize "(X=1.000000,Y=1.000000)" :BlendMode "BLEND_Opaque" :PivotPoint "(X=0.500000,Y=0.500000)")
      (Rendering|EndDrawCanvastoRenderTarget _context))
    (:then_1
      ;[0.15 0.15 0.15 0.5] Raycast
      (bind (_hitlocation _hitnormal _bonename _outhit _returnvalue_2) (Collision|LineTraceComponent (Variables|Default|GetStaticMesh) _returnvalue (+ _returnvalue (* (Transformation|GetActorUpVector _drawtool) 1e+02)) true true false))
      (if _returnvalue_2
        ;[0.15 0.15 0.15 0.5] Check for collision and pass col-info in UV-space to material instance
        (Rendering|Material|SetVectorParameterValue (Variables|State|GetInstanceBrushMaterial) "BrushPositionUV" (Utilities|Struct|MakeLinearColor (.x (.UV (Class|GameplayStatics|FindCollisionUV _outhit))) (.y (.UV (Class|GameplayStatics|FindCollisionUV _outhit))) (Math|Conversions|ToFloat(Boolean) (.ReturnValue (Class|GameplayStatics|FindCollisionUV _outhit))) 1.0) :!class /Script/Engine.MaterialInstanceDynamic)
        ;[0.15 0.15 0.15 0.5] Update and confirm changes on material
        (bind (_canvas_2 _size_2 _context_2) (Rendering|BeginDrawCanvastoRenderTarget (Variables|State|GetPaintingRenderTargetCopy)))
        (Canvas|DrawMaterial :self _canvas_2 :RenderMaterial (Variables|State|GetInstanceBrushMaterial) :ScreenSize _size_2 :CoordinateSize "(X=1.000000,Y=1.000000)" :PivotPoint "(X=0.500000,Y=0.500000)")
        (Rendering|EndDrawCanvastoRenderTarget _context_2)))))

(fn ConstructionScript)

(fn Setup
  (bind _paintingrendertarget (Variables|Settings|GetPaintingRenderTarget))
  (Utilities|FlowControl|Sequence
    (:then_0
      ;[0.15 0.15 0.15 0.5] Clear RenderTarget from previous drawings
      (Rendering|ClearRenderTarget2D (Variables|Settings|GetPaintingRenderTarget)))
    (:then_1
      ;[0.15 0.15 0.15 0.5] Create Dynamic Material Instance and set it's RenderTarget parameter
      (bind _returnvalue (Rendering|Material|CreateDynamicMaterialInstance (Variables|Settings|GetBaseBrushMaterial) "BrushMatInstance" "None" :!class /Script/Engine.KismetMaterialLibrary))
      (bind _output_get (Variables|State|SetInstanceBrushMaterial _returnvalue))
      (Rendering|Material|SetTextureParameterValue _output_get "RenderTarget" (Variables|Settings|GetPaintingRenderTarget)))
    (:then_2
      ;[0.15 0.15 0.15 0.5] Create copy of Render Target, to keep previous drawings
      (bind _returnvalue_2 (Rendering|CreateRenderTarget2D (Variables|/Script/Engine.TextureRenderTarget2D|GetSizeX _paintingrendertarget) (Variables|/Script/Engine.TextureRenderTarget2D|GetSizeY _paintingrendertarget) (Variables|/Script/Engine.TextureRenderTarget2D|GetRenderTargetFormat _paintingrendertarget) (Variables|/Script/Engine.TextureRenderTarget2D|GetClearColor _paintingrendertarget) (Variables|/Script/Engine.TextureRenderTarget2D|GetbAutoGenerateMips _paintingrendertarget) (Variables|/Script/Engine.TextureRenderTarget2D|GetbSupportsUAV _paintingrendertarget)))
      (Variables|State|SetPaintingRenderTargetCopy _returnvalue_2))
    (:then_3
      (bind _returnvalue_3 (Actor|GetActorOfClass "/Game/Blueprints/HapticFeedback/BP_HapticTool.BP_HapticTool_C"))
      (Variables|Settings|SetDrawTool _returnvalue_3))))