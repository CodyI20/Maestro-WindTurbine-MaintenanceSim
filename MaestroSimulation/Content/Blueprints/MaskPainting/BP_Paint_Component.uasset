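; Component that lets the player paint a mask onto static meshes tagged "Paint" and detects when they are covered.
; UpdatePainting stamps a brush material at the hit's collision UV, with Scale-driven flow, using a render-target copy to preserve earlier strokes.
; A cooldown-throttled fill check compares painted coverage to a threshold, then fires completion, disables the outline and starts Tick-driven glow pulses and auto-fill.
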(event EventBeginPlay
  (CallFunction|Setup))

(event EventTick
  (params (DeltaSeconds :type Float%20%28single-precision%29))
  (Glow|UpdateFillCheckTimer)
  (Glow|UpdateGlow)
  (AutoFill|UpdateFillRT))

(fn Setup
  (bind _paintingrendertarget (Variables|Settings|GetPaintingRenderTarget))
  (Utilities|FlowControl|Sequence
    (:then_0
      ;[0.15 0.15 0.15 0.5] Clear RenderTarget from previous drawings
      (Rendering|ClearRenderTarget2D (Variables|Settings|GetPaintingRenderTarget))
      (Rendering|ClearRenderTarget2D (Variables|Settings|GetFillRenderTarget)))
    (:then_1
      ;[0.15 0.15 0.15 0.5] Create Dynamic Material Instance and set it's RenderTarget parameter
      (bind _returnvalue (Rendering|Material|CreateDynamicMaterialInstance (Variables|Settings|GetBaseBrushMaterial) "BrushMatInstance" "None" :!class /Script/Engine.KismetMaterialLibrary))
      (bind _output_get (Variables|State|SetInstanceBrushMaterial _returnvalue))
      (Rendering|Material|SetTextureParameterValue _output_get "RenderTarget" (Variables|Settings|GetPaintingRenderTarget)))
    (:then_2
      ;[0.15 0.15 0.15 0.5] Create copy of Render Target, to keep previous drawings
      (bind _returnvalue_2 (Rendering|CreateRenderTarget2D (Variables|/Script/Engine.TextureRenderTarget2D|GetSizeX _paintingrendertarget) (Variables|/Script/Engine.TextureRenderTarget2D|GetSizeY _paintingrendertarget) (Variables|/Script/Engine.TextureRenderTarget2D|GetRenderTargetFormat _paintingrendertarget) (Variables|/Script/Engine.TextureRenderTarget2D|GetClearColor _paintingrendertarget) (Variables|/Script/Engine.TextureRenderTarget2D|GetbAutoGenerateMips _paintingrendertarget) (Variables|/Script/Engine.TextureRenderTarget2D|GetbSupportsUAV _paintingrendertarget)))
      (Variables|State|SetPaintingRenderTargetCopy _returnvalue_2))
    (:then_3
      ;[0.15 0.15 0.15 0.5] Get all needed component references
      (bind _returnvalue_3 (Actor|GetActorOfClass "/Game/Blueprints/BristleBlaster/BP_BristleBlaster.BP_BristleBlaster_C"))
      (Variables|Settings|SetHapticTool _returnvalue_3)
      (bind _outactors (Actor|GetAllActorswithTag "Paint"))
      (for _array_element _outactors
        (Utilities|Array|AppendArray (Variables|Default|GetPaintingStaticMesh) (Actor|GetComponentsbyTag _array_element "/Script/Engine.StaticMeshComponent" "Paint"))
        ;[0.15 0.15 0.15 0.5] Applies the glow texture
        (for (_array_element_2 _array_index) (Actor|GetComponentsbyTag _array_element "/Script/Engine.StaticMeshComponent" "Paint")
          (bind _asmaterial_instance_dynamic (Utilities|Casting|CastToMaterialInstanceDynamic (Rendering|Material|GetMaterial _array_element_2 0))
            (:then
              (Utilities|Array|Add (Variables|Glow|GetDrawnUponMaterial) _asmaterial_instance_dynamic))
            (:CastFailed
              (bind _returnvalue_4 (Rendering|Material|CreateDynamicMaterialInstance (Rendering|Material|GetMaterial _array_element_2 0) (Utilities|Name|MakeLiteralName (Utilities|String|StringToName (Utilities|String|MakeLiteralString (Utilities|String|ToString(Text) (Utilities|Text|FormatText "CanvasMaterialInstance{Index}" _array_index))))) "None" :!class /Script/Engine.KismetMaterialLibrary))
              (Utilities|Array|Add (Variables|Glow|GetDrawnUponMaterial) _returnvalue_4)
              (Rendering|Material|SetMaterial _array_element_2 0 _returnvalue_4))))))
    (:then_4
      ;[0.15 0.15 0.15 0.5] Setup count of canvases
      (Variables|Default|SetDrawCanvasCount (- (Utilities|Array|Length (Variables|Glow|GetDrawnUponMaterial)) 1))
      ;[0.15 0.15 0.15 0.5] Setup Glow values
      (Variables|Glow|SetGlowPerSecond (/ (Variables|Glow|GetMaxGlow) (Variables|Glow|GetSecondsToGlowUp)))
      ;[0.15 0.15 0.15 0.5] Setup Fill Speed
      (Variables|AutoFill|SetFillPerSecond (/ (Variables|AutoFill|GetMaxFill) (Variables|AutoFill|GetSecondsToFill))))
    (:then_5
      ;[0.15 0.15 0.15 0.5] Setup arrays
      (for _index (range 0 (Variables|Default|GetDrawCanvasCount))
        (Utilities|Array|Add (Variables|Glow|GetApplyGlow) false)
        (Utilities|Array|Add (Variables|Glow|GetGlowUp) false)
        (Utilities|Array|Add (Variables|Glow|GetGlowComplete) false)
        (Utilities|Array|Add (Variables|Glow|GetTimerCooldown) (Variables|Glow|GetMaxTimerCooldown))
        (Utilities|Array|Add (Variables|Glow|GetCurrentGlow) 0.0)))))

(fn UpdatePainting
  (params (Scale :type Float%20%28double-precision%29) (Hit :type Hit%20Result%20Structure))
  (bind _instancebrushmaterial (Variables|State|GetInstanceBrushMaterial))
  (bind (_uv _returnvalue) (Class|GameplayStatics|FindCollisionUV Hit))
  ;[0.15 0.15 0.15 0.5] Update the copy of the material instance
  (Utilities|FlowControl|Sequence
    (:then_0
      (bind (_canvas _size _context) (Rendering|BeginDrawCanvastoRenderTarget (Variables|Settings|GetPaintingRenderTarget)))
      (Canvas|DrawTexture :self _canvas :RenderTexture (Variables|State|GetPaintingRenderTargetCopy) :ScreenSize _size :CoordinateSize "(X=1.000000,Y=1.000000)" :BlendMode "BLEND_Opaque" :PivotPoint "(X=0.500000,Y=0.500000)")
      (Rendering|EndDrawCanvastoRenderTarget _context)
      ;[0.15 0.15 0.15 0.5] Map scaling value to adjust opacity more appropriately
      (if (> Scale 0.5)
        (LocalVariables|SetAdjustedScale (Math|Float|MapRangeClamped Scale 0.5 1.0 0.1 0.3))
        (else
          (LocalVariables|SetAdjustedScale (Math|Float|MapRangeClamped Scale 0.0 0.5 0.005 0.1)))))
    (:then_1
      ;[0.15 0.15 0.15 0.5] Check if hit component is painting canvas
      (bind _asstatic_mesh_component (Utilities|Casting|CastToStaticMeshComponent (.HitComponent (Collision|BreakHitResult Hit)))
        (:then
          (if (Utilities|Array|ContainsItem (Variables|Default|GetPaintingStaticMesh) _asstatic_mesh_component)
            ;[0.15 0.15 0.15 0.5] Check for collision and pass col-info in UV-space to material instance
            (Rendering|Material|SetVectorParameterValue _instancebrushmaterial "BrushPositionUV" (Utilities|Struct|MakeLinearColor (.x _uv) (.y _uv) (Math|Conversions|ToFloat(Boolean) _returnvalue) 1.0) :!class /Script/Engine.MaterialInstanceDynamic)
            ;[0.15 0.15 0.15 0.5] Set painting opacity based on scale
            (Rendering|Material|SetScalarParameterValue _instancebrushmaterial "BrushFlow" (LocalVariables|GetAdjustedScale) :!class /Script/Engine.MaterialInstanceDynamic)
            ;[0.15 0.15 0.15 0.5] Update and confirm changes on material
            (bind (_canvas_2 _size_2 _context_2) (Rendering|BeginDrawCanvastoRenderTarget (Variables|State|GetPaintingRenderTargetCopy)))
            (Canvas|DrawMaterial :self _canvas_2 :RenderMaterial (Variables|State|GetInstanceBrushMaterial) :ScreenSize _size_2 :CoordinateSize "(X=1.000000,Y=1.000000)" :PivotPoint "(X=0.500000,Y=0.500000)")
            (Rendering|EndDrawCanvastoRenderTarget _context_2)
            ;[0.15 0.15 0.15 0.5] If timer completed, check if area is filled
            (for _index (range 0 (Variables|Default|GetDrawCanvasCount))
              (if (<= (Utilities|Array|Get(acopy) (Variables|Glow|GetTimerCooldown) _index) 0.0)
                (Glow|CheckifFilled))
              (Utilities|FlowControl|Sequence
                (:then_0
                  (Utilities|FlowControl|DoOnce false
                    (:Completed
                      (bind _ascustom_game_instance (Utilities|Casting|CastToBP_WindTurbine_GameInstance (Game|GetGameInstance)))
                      (Default|CallMaskPaintingComplete _ascustom_game_instance))))
                (:then_1
                  (return true))))
            (else
              (return false))))
        (:CastFailed
          (return false))))))

(fn CheckifFilled
  (for _index (range 0 (Variables|Default|GetDrawCanvasCount))
    (bind _output_get (LocalVariables|SetIndex _index))
    (if (not (Utilities|Array|Get(acopy) (Variables|Glow|GetApplyGlow) _output_get))
      (bind _returnvalue (Class|RTReader|GetRTFillPercent "/Game/Materials/MaskPainting/Textures/RT_Painting.RT_Painting"))
      (Utilities|Array|SetArrayElem (Variables|Glow|GetTimerCooldown) (LocalVariables|GetIndex) (Variables|Glow|GetMaxTimerCooldown))
      (if (>= (/ _returnvalue 0.004654) (Variables|AutoFill|GetFillThreshold))
        (Utilities|Array|SetArrayElem (Variables|Glow|GetApplyGlow) (LocalVariables|GetIndex) true)
        (Utilities|Array|SetArrayElem (Variables|Glow|GetGlowUp) (LocalVariables|GetIndex) true)
        (Variables|AutoFill|SetIsAutoFillActive true)
        (Rendering|Material|SetScalarParameterValue (Utilities|Array|Get(acopy) (Variables|Glow|GetDrawnUponMaterial) (LocalVariables|GetIndex)) "DeactivateOutline" 1.0 :!class /Script/Engine.MaterialInstanceDynamic)
        (Default|CallOnPaintComplete)))))

(fn UpdateGlow
  (bind _returnvalue (Utilities|Time|GetWorldDeltaSeconds))
  (bind _glowpersecond (Variables|Glow|GetGlowPerSecond))
  (bind _returnvalue_2 (* _glowpersecond _returnvalue))
  (for _index (range 0 (Variables|Default|GetDrawCanvasCount))
    (LocalVariables|SetIndex _index)
    (if (and (Utilities|Array|Get(acopy) (Variables|Glow|GetApplyGlow) (LocalVariables|GetIndex)) (not (Utilities|Array|Get(acopy) (Variables|Glow|GetGlowComplete) (LocalVariables|GetIndex))))
      (if (Utilities|Array|Get(acopy) (Variables|Glow|GetGlowUp) (LocalVariables|GetIndex))
        (Utilities|Array|SetArrayElem (Variables|Glow|GetCurrentGlow) (LocalVariables|GetIndex) (Math|Float|Clamp(Float) (+ (Utilities|Array|Get(acopy) (Variables|Glow|GetCurrentGlow) (LocalVariables|GetIndex)) _returnvalue_2) 0.0 (Variables|Glow|GetMaxGlow)))
        (Rendering|Material|SetScalarParameterValue (Utilities|Array|Get(acopy) (Variables|Glow|GetDrawnUponMaterial) (LocalVariables|GetIndex)) "GlowScale" (Math|Float|Clamp(Float) (+ (Utilities|Array|Get(acopy) (Variables|Glow|GetCurrentGlow) (LocalVariables|GetIndex)) _returnvalue_2) 0.0 (Variables|Glow|GetMaxGlow)) :!class /Script/Engine.MaterialInstanceDynamic)
        (if (>= (Utilities|Array|Get(acopy) (Variables|Glow|GetCurrentGlow) (LocalVariables|GetIndex)) (Variables|Glow|GetMaxGlow))
          (Utilities|Array|SetArrayElem (Variables|Glow|GetGlowUp) (LocalVariables|GetIndex) false))
        (else
          (Utilities|Array|SetArrayElem (Variables|Glow|GetCurrentGlow) (LocalVariables|GetIndex) (- (Utilities|Array|Get(acopy) (Variables|Glow|GetCurrentGlow) (LocalVariables|GetIndex)) _returnvalue_2))
          (Rendering|Material|SetScalarParameterValue (Utilities|Array|Get(acopy) (Variables|Glow|GetDrawnUponMaterial) (LocalVariables|GetIndex)) "GlowScale" (- (Utilities|Array|Get(acopy) (Variables|Glow|GetCurrentGlow) (LocalVariables|GetIndex)) _returnvalue_2) :!class /Script/Engine.MaterialInstanceDynamic)
          (if (<= (Utilities|Array|Get(acopy) (Variables|Glow|GetCurrentGlow) (LocalVariables|GetIndex)) 0.0)
            (Variables|Glow|SetCurrentGlowUpCount (+ (Variables|Glow|GetCurrentGlowUpCount) 1))
            (if (< (Variables|Glow|GetCurrentGlowUpCount) (Variables|Glow|GetMaxGlowCount))
              (Utilities|Array|SetArrayElem (Variables|Glow|GetGlowUp) (LocalVariables|GetIndex) true)
              (else
                (Utilities|Array|SetArrayElem (Variables|Glow|GetGlowComplete) (LocalVariables|GetIndex) false)))))))))

(fn UpdateFillCheckTimer
  (for _index (range 0 (Variables|Default|GetDrawCanvasCount))
    (LocalVariables|SetIndex _index)
    (if (> (Utilities|Array|Get(acopy) (Variables|Glow|GetTimerCooldown) (LocalVariables|GetIndex)) 0.0)
      (Utilities|Array|SetArrayElem (Variables|Glow|GetTimerCooldown) (LocalVariables|GetIndex) (- (Utilities|Array|Get(acopy) (Variables|Glow|GetTimerCooldown) (LocalVariables|GetIndex)) (Utilities|Time|GetWorldDeltaSeconds))))))

(fn UpdateFillRT
  (if (and (Variables|AutoFill|GetIsAutoFillActive) (< (Variables|AutoFill|GetCurrentFill) (Variables|AutoFill|GetMaxFill)))
    (bind _output_get (Variables|AutoFill|SetCurrentFill (Math|Float|Clamp(Float) (+ (* (Variables|AutoFill|GetFillPerSecond) (Utilities|Time|GetWorldDeltaSeconds)) (Variables|AutoFill|GetCurrentFill)) 0.0 (Variables|AutoFill|GetMaxFill))))
    (Rendering|ClearRenderTarget2D (Variables|Settings|GetFillRenderTarget) (Math|Color|MakeColor _output_get 0.0 0.0))))