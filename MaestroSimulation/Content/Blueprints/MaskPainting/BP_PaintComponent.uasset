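; Paint component that lets brush hits paint onto "Paint"-tagged static meshes and makes the painted surface glow once sufficiently filled.
; UpdatePainting converts hits to UVs and draws a brush material, with scale-driven flow, between a render target and its copy to retain strokes.
; A cooldown throttles fill-percentage checks during painting.
; Passing the threshold starts Tick-driven GlowScale pulses on the last tagged mesh's dynamic material.
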(event EventBeginPlay
  (CallFunction|Setup))

(event EventTick
  (params (DeltaSeconds :type Float%20%28single-precision%29))
  (Glow|UpdateFillCheckTimer)
  (Glow|UpdateGlow))

(fn Setup
  (bind _paintingrendertarget (Variables|Settings|GetPaintingRenderTarget))
  (Utilities|FlowControl|Sequence
    (:then_0
      ;[0.15 0.15 0.15 0.5] Clear RenderTarget from previous drawings
      (Rendering|ClearRenderTarget2D (Variables|Settings|GetPaintingRenderTarget)))
    (:then_1
      ;[0.15 0.15 0.15 0.5] Create Dynamic Material Instance and set it's RenderTarget parameter
      (bind _returnvalue (Rendering|Material|CreateDynamicMaterialInstance (Variables|Settings|GetBaseBrushMaterial) "BrushMatInstance" "None" :!class /Script/Engine.KismetMaterialLibrary))
      (bind _output_get (Variables|State|SetInstanceBrushMaterial _returnvalue))
      (Rendering|Material|SetTextureParameterValue _output_get "RenderTarget" (Variables|Settings|GetPaintingRenderTarget)))
    (:then_2
      ;[0.15 0.15 0.15 0.5] Create copy of Render Target, to keep previous drawings
      (bind _returnvalue_2 (Rendering|CreateRenderTarget2D (Variables|/Script/Engine.TextureRenderTarget2D|GetSizeX _paintingrendertarget) (Variables|/Script/Engine.TextureRenderTarget2D|GetSizeY _paintingrendertarget) (Variables|/Script/Engine.TextureRenderTarget2D|GetRenderTargetFormat _paintingrendertarget) (Variables|/Script/Engine.TextureRenderTarget2D|GetClearColor _paintingrendertarget) (Variables|/Script/Engine.TextureRenderTarget2D|GetbAutoGenerateMips _paintingrendertarget) (Variables|/Script/Engine.TextureRenderTarget2D|GetbSupportsUAV _paintingrendertarget)))
      (Variables|State|SetPaintingRenderTargetCopy _returnvalue_2))
    (:then_3
      ;[0.15 0.15 0.15 0.5] Get all needed component references
      (bind _returnvalue_3 (Actor|GetActorOfClass "/Game/Blueprints/HapticFeedback/BP_HapticTool.BP_HapticTool_C"))
      (Variables|Settings|SetHapticTool _returnvalue_3)
      (bind _outactors (Actor|GetAllActorswithTag "Paint"))
      (for _array_element _outactors
        (Utilities|Array|AppendArray (Variables|Default|GetPaintingStaticMesh) (Actor|GetComponentsbyTag _array_element "/Script/Engine.StaticMeshComponent" "Paint"))
        ;[0.15 0.15 0.15 0.5] Though it goes through the whole array, it will only consider the last index item. We have no need for multiple different glows
        (for _array_element_2 (Actor|GetComponentsbyTag _array_element "/Script/Engine.StaticMeshComponent" "Paint")
          (bind _output_get_2 (Variables|Settings|SetBaseDrawnMaterial (Rendering|Material|GetMaterial _array_element_2 0)))
          (bind _returnvalue_4 (Rendering|Material|CreateDynamicMaterialInstance _output_get_2 "DrawnMatInstance" "None" :!class /Script/Engine.KismetMaterialLibrary))
          (bind _output_get_3 (Variables|Glow|SetDrawnUponMaterial _returnvalue_4))
          (Rendering|Material|SetMaterial _array_element_2 0 _output_get_3))))
    (:then_4
      ;[0.15 0.15 0.15 0.5] Setup Fill check & Glow values
      (Variables|Glow|SetTimerCooldown (Variables|Glow|GetMaxTimerCooldown))
      (Variables|Glow|SetGlowPerSecond (/ (Variables|Glow|GetMaxGlow) (Variables|Glow|GetSecondsToGlowUp))))))

(fn UpdatePainting
  (params (Scale :type Float%20%28double-precision%29) (Hit :type Hit%20Result%20Structure))
  (bind _instancebrushmaterial (Variables|State|GetInstanceBrushMaterial))
  (bind (_uv _returnvalue) (Class|GameplayStatics|FindCollisionUV Hit))
  ;[0.15 0.15 0.15 0.5] Update the copy of the material instance
  (Utilities|FlowControl|Sequence
    (:then_0
      (bind (_canvas _size _context) (Rendering|BeginDrawCanvastoRenderTarget (Variables|Settings|GetPaintingRenderTarget)))
      (Canvas|DrawTexture :self _canvas :RenderTexture (Variables|State|GetPaintingRenderTargetCopy) :ScreenSize _size :CoordinateSize "(X=1.000000,Y=1.000000)" :BlendMode "BLEND_Opaque" :PivotPoint "(X=0.500000,Y=0.500000)")
      (Rendering|EndDrawCanvastoRenderTarget _context)
      ;[0.15 0.15 0.15 0.5] Map scaling value to adjust opacity more appropriately
      (if (> Scale 0.5)
        (LocalVariables|SetAdjustedScale (Math|Float|MapRangeClamped Scale 0.5 1.0 0.1 0.3))
        (else
          (LocalVariables|SetAdjustedScale (Math|Float|MapRangeClamped Scale 0.0 0.5 0.005 0.1)))))
    (:then_1
      ;[0.15 0.15 0.15 0.5] Check if hit component is painting canvas
      (bind _asstatic_mesh_component (Utilities|Casting|CastToStaticMeshComponent (.HitComponent (Collision|BreakHitResult Hit)))
        (:then
          (if (Utilities|Array|ContainsItem (Variables|Default|GetPaintingStaticMesh) _asstatic_mesh_component)
            ;[0.15 0.15 0.15 0.5] Check for collision and pass col-info in UV-space to material instance
            (Rendering|Material|SetVectorParameterValue _instancebrushmaterial "BrushPositionUV" (Utilities|Struct|MakeLinearColor (.x _uv) (.y _uv) (Math|Conversions|ToFloat(Boolean) _returnvalue) 1.0) :!class /Script/Engine.MaterialInstanceDynamic)
            ;[0.15 0.15 0.15 0.5] Set painting opacity based on scale
            (Rendering|Material|SetScalarParameterValue _instancebrushmaterial "BrushFlow" (LocalVariables|GetAdjustedScale) :!class /Script/Engine.MaterialInstanceDynamic)
            ;[0.15 0.15 0.15 0.5] Update and confirm changes on material
            (bind (_canvas_2 _size_2 _context_2) (Rendering|BeginDrawCanvastoRenderTarget (Variables|State|GetPaintingRenderTargetCopy)))
            (Canvas|DrawMaterial :self _canvas_2 :RenderMaterial (Variables|State|GetInstanceBrushMaterial) :ScreenSize _size_2 :CoordinateSize "(X=1.000000,Y=1.000000)" :PivotPoint "(X=0.500000,Y=0.500000)")
            (Rendering|EndDrawCanvastoRenderTarget _context_2)
            ;[0.15 0.15 0.15 0.5] If timer completed, check if area is filled
            (if (<= (Variables|Glow|GetTimerCooldown) 0.0)
              (Glow|CheckifFilled))
            (return true)
            (else
              _)))
        (:CastFailed
          _))
      (return false))))

(fn CheckifFilled
  (if (not (Variables|Glow|GetApplyGlow))
    (bind _returnvalue (Class|RTReader|GetRTFillPercent "/Game/Blueprints/MaskPainting/RT_Painting.RT_Painting"))
    (Variables|Glow|SetTimerCooldown (Variables|Glow|GetMaxTimerCooldown))
    (if (>= (/ _returnvalue 0.004654) (Variables|Glow|GetFillThreshold))
      (Variables|Glow|SetApplyGlow true)
      (Variables|Glow|SetGlowUp true))))

(fn UpdateGlow
  (bind _returnvalue (Utilities|Time|GetWorldDeltaSeconds))
  (bind _glowpersecond (Variables|Glow|GetGlowPerSecond))
  (bind _returnvalue_2 (* _glowpersecond _returnvalue))
  (if (and (Variables|Glow|GetApplyGlow) (not (Variables|Glow|GetGlowComplete)))
    (if (Variables|Glow|GetGlowUp)
      (Variables|Glow|SetCurrentGlow (Math|Float|Clamp(Float) (+ (Variables|Glow|GetCurrentGlow) _returnvalue_2) 0.0 (Variables|Glow|GetMaxGlow)))
      (Rendering|Material|SetScalarParameterValue (Variables|Glow|GetDrawnUponMaterial) "GlowScale" (Math|Float|Clamp(Float) (+ (Variables|Glow|GetCurrentGlow) _returnvalue_2) 0.0 (Variables|Glow|GetMaxGlow)) :!class /Script/Engine.MaterialInstanceDynamic)
      (if (>= (Variables|Glow|GetCurrentGlow) (Variables|Glow|GetMaxGlow))
        (Variables|Glow|SetGlowUp false))
      (else
        (Variables|Glow|SetCurrentGlow (- (Variables|Glow|GetCurrentGlow) _returnvalue_2))
        (Rendering|Material|SetScalarParameterValue (Variables|Glow|GetDrawnUponMaterial) "GlowScale" (- (Variables|Glow|GetCurrentGlow) _returnvalue_2) :!class /Script/Engine.MaterialInstanceDynamic)
        (if (<= (Variables|Glow|GetCurrentGlow) 0.0)
          (Variables|Glow|SetCurrentGlowUpCount (+ (Variables|Glow|GetCurrentGlowUpCount) 1))
          (if (< (Variables|Glow|GetCurrentGlowUpCount) (Variables|Glow|GetMaxGlowCount))
            (Variables|Glow|SetGlowUp true)
            (else
              (Variables|Glow|SetGlowComplete false))))))))

(fn UpdateFillCheckTimer
  (if (> (Variables|Glow|GetTimerCooldown) 0.0)
    (Variables|Glow|SetTimerCooldown (- (Variables|Glow|GetTimerCooldown) (Utilities|Time|GetWorldDeltaSeconds)))))