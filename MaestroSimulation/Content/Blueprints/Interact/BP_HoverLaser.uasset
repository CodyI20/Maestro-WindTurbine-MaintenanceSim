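; BP_HoverLaser provides laser-pointer hovering for left and right controllers, with a Niagara beam and a cursor.
; HoverCheck line-traces forward to the interaction distance, tracks a hovered actor per hand, and sends begin and end hover messages through BPI_Interactable.
; UpdateLaserAndCursor writes beam endpoints into the Niagara point array, placing the cursor on hits.
; Without a hit, it hides both, or only the cursor when the laser is always visible.
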(fn LaserCursorVisibility
  (params (Visibility :type Boolean) (Laser :type Niagara%20Component%20Object%20Reference) (Cursor :type Static%20Mesh%20Component%20Object%20Reference))
  (Rendering|SetVisibility Laser Visibility false)
  (Rendering|SetVisibility Cursor Visibility false))

(fn UpdateLaserandCursor
  (params (LaserAlwaysVisible :type Boolean) (HitFromRaycast :type Boolean) (ObjectLaserComesFrom :type Widget%20Interaction%20Component%20Object%20Reference) (Cursor :type Static%20Mesh%20Component%20Object%20Reference) (Laser :type Niagara%20Component%20Object%20Reference) (HitLocation :type Vector))
  (if (or LaserAlwaysVisible HitFromRaycast)
    (CallFunction|LaserCursorVisibility true Laser Cursor)
    (Variables|Default|SetLaserStartPoint (Transformation|GetWorldLocation ObjectLaserComesFrom))
    (if HitFromRaycast
      (Variables|Default|SetLaserEndPoint HitLocation)
      (Transformation|SetWorldLocation Cursor (Variables|Default|GetLaserEndPoint) false false)
      (else
        (Variables|Default|SetLaserEndPoint (|FindEndofWidgetInteractionComponent_2 ObjectLaserComesFrom))
        (Rendering|SetVisibility Cursor false false)))
    (Class|NiagaraDataInterfaceArrayFunctionLibrary|SetNiagaraArrayVectorValue Laser "User.PointArray" 0 (Variables|Default|GetLaserStartPoint) false)
    (Class|NiagaraDataInterfaceArrayFunctionLibrary|SetNiagaraArrayVectorValue Laser "User.PointArray" 1 (Variables|Default|GetLaserEndPoint) false)
    (else
      (CallFunction|LaserCursorVisibility false Laser Cursor))))

(fn HoverCheck
  (params (ObjectToTraceLineFrom :type Widget%20Interaction%20Component%20Object%20Reference) (IsLeftController :type Boolean))
  (bind _returnvalue (Transformation|GetWorldTransform ObjectToTraceLineFrom))
  (bind (_outhit _returnvalue_2) (Collision|LineTraceByChannel (.location _returnvalue) (+ (.location _returnvalue) (* (Math|Vector|GetForwardVector (.rotation _returnvalue)) (Variables|/Script/UMG.WidgetInteractionComponent|GetInteractionDistance ObjectToTraceLineFrom))) "TraceTypeQuery4" false 0 "None"))
  (if _returnvalue_2
    (if (Utilities|DoesObjectImplementInterface (.HitActor (Collision|BreakHitResult _outhit)) "/Game/Blueprints/Interact/BPI_Interactable.BPI_Interactable_C")
      (if IsLeftController
        (bind _lefthoveredactor (Variables|Default|GetLeftHoveredActor)
          (:then
            (if (== _lefthoveredactor (.HitActor (Collision|BreakHitResult _outhit)))
              (if (not (Variables|Default|GetIsLeftHovered)) :!label _label
                (bind _output_get (Variables|Default|SetLeftHoveredActor (.HitActor (Collision|BreakHitResult _outhit)) :!label _label_2))
                (Class|BPIInteractable|OnBeginHover(Message) _output_get)
                (return _returnvalue_2 (.ImpactPoint (Collision|BreakHitResult _outhit))))
              (else
                (Class|BPIInteractable|OnEndHover(Message) _lefthoveredactor)
                (Variables|Default|SetIsLeftHovered false)
                (goto _label_2))))
          (:else
            (goto _label)))
        (else
          (bind _righthoveredactor (Variables|Default|GetRightHoveredActor)
            (:then
              (if (== _righthoveredactor (.HitActor (Collision|BreakHitResult _outhit)))
                (if (not (Variables|Default|GetIsRightHovered)) :!label _label_3
                  (bind _output_get_2 (Variables|Default|SetRightHoveredActor (.HitActor (Collision|BreakHitResult _outhit)) :!label _label_4))
                  (Class|BPIInteractable|OnBeginHover(Message) _output_get_2)
                  (return _returnvalue_2 (.ImpactPoint (Collision|BreakHitResult _outhit))))
                (else
                  (Class|BPIInteractable|OnEndHover(Message) _righthoveredactor)
                  (Variables|Default|SetIsRightHovered false)
                  (goto _label_4))))
            (:else
              (goto _label_3))))))
    (else
      (if IsLeftController
        (bind _lefthoveredactor_2 (Variables|Default|GetLeftHoveredActor)
          (:then
            (Class|BPIInteractable|OnEndHover(Message) _lefthoveredactor_2)
            (Variables|Default|SetLeftHoveredActor 0)
            (Variables|Default|SetIsLeftHovered false)
            (return _returnvalue_2 (.ImpactPoint (Collision|BreakHitResult _outhit))))
          (:else
            _))
        (else
          (bind _righthoveredactor_2 (Variables|Default|GetRightHoveredActor)
            (:then
              (Class|BPIInteractable|OnEndHover(Message) _righthoveredactor_2)
              (Variables|Default|SetRightHoveredActor 0)
              (Variables|Default|SetIsRightHovered false)
              (return _returnvalue_2 (.ImpactPoint (Collision|BreakHitResult _outhit))))
            (:else
              _))))
      (return _returnvalue_2 (.TraceEnd (Collision|BreakHitResult _outhit))))))