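; Physics-simulated cable actor that renders a chain of constrained bodies as a smooth rope.
; The construction script spawns static mesh links with the first one non-simulated, joins neighbors with physics constraints, and creates spline points and spline mesh segments.
; Tick moves spline points to the links, then bends segments along the spline at MeshLength intervals, separating physics from visuals.
; Setup, which zeroes link velocities, is never called.
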(event EventBeginPlay)

(event Collision|EventActorBeginOverlap
  (params (OtherActor :type Actor%20Object%20Reference)))

(event EventTick
  (params (DeltaSeconds :type Float%20%28single-precision%29))
  (bind _spline (Variables|Default|GetSpline))
  (bind _spline_2 (Variables|Default|GetSpline))
  (Utilities|FlowControl|Sequence
    (:then_0
      (for (_array_element _array_index) (Variables|Default|GetLinks)
        (Spline|SetLocationatSplinePoint (Variables|Default|GetSpline) _array_index (Transformation|GetWorldLocation _array_element) "World" true)))
    (:then_1
      (for (_array_element_2 _array_index_2) (Variables|Default|GetSplineMeshSegments)
        (SplineMesh|SetStartandEnd _array_element_2 (Spline|GetLocationatDistanceAlongSpline _spline_2 (* _array_index_2 (Variables|Default|GetMeshLength)) "Local") (Spline|GetTangentatDistanceAlongSpline _spline_2 (* _array_index_2 (Variables|Default|GetMeshLength)) "Local") (Spline|GetLocationatDistanceAlongSpline _spline (* (+ _array_index_2 1) (Variables|Default|GetMeshLength)) "Local") (Spline|GetTangentatDistanceAlongSpline _spline (* (+ _array_index_2 1) (Variables|Default|GetMeshLength)) "Local") true :!class /Script/Engine.SplineMeshComponent)))))

(fn ConstructionScript
  (bind _links (Variables|Default|GetLinks))
  (for _index (range 0 (- (Variables|Default|GetNumLinks) 1))
    (Utilities|FlowControl|Sequence
      (:then_0
        ;[0.15 0.15 0.15 0.5] Add static meshes and set simulate physics for all, but the first component added. This however is not the visible mesh itself, but rather a physics reference point
        (bind _returnvalue (AddComponent|AddStaticMeshComponent false))
        (Physics|SetSimulatePhysics _returnvalue (!= 0 _index))
        (Transformation|AttachComponentToComponent _returnvalue (Variables|Default|GetSpline) "None" "KeepWorld" "KeepWorld" "KeepWorld" false)
        (Transformation|SetRelativeLocation _returnvalue (Math|Vector|MakeVector (Math|Conversions|ToFloat(Integer) (* _index 20)) 0.0 0.0) false false)
        (Utilities|Array|Add (Variables|Default|GetLinks) _returnvalue))
      (:then_1
        ;[0.15 0.15 0.15 0.5] Add physics constraint to every added static mesh. This is what makes the rope behaviour work
        (if (> _index 0)
          (bind _returnvalue_2 (AddComponent|AddPhysicsConstraintComponent false))
          (Transformation|SetRelativeLocation _returnvalue_2 (Math|Vector|MakeVector (Math|Conversions|ToFloat(Integer) (* _index 20)) 0.0 0.0) false false)
          (Class|PhysicsConstraintComponent|SetConstrainedComponents _returnvalue_2 (Utilities|Array|Get(acopy) _links (- _index 1)) "None" (Utilities|Array|Get(acopy) _links _index) "None")
          (Utilities|Array|Add (Variables|Default|GetConstraints) _returnvalue_2)))))
  ;[0.15 0.15 0.15 0.5] Reset spline and add all points with a cylinder mesh. This handles the visual part of the rope, connecting it smoothly
  (Spline|ClearSplinePoints (Variables|Default|GetSpline) true)
  (for _array_element (Variables|Default|GetLinks)
    (Spline|AddSplinePoint (Variables|Default|GetSpline) (Transformation|GetWorldLocation _array_element) "World" true)
    (bind _returnvalue_3 (AddComponent|AddSplineMeshComponent false))
    (Transformation|AttachComponentToComponent _returnvalue_3 (Variables|Default|GetSpline) "None" "KeepRelative" "KeepRelative" "KeepRelative" false)
    (Utilities|Array|Add (Variables|Default|GetSplineMeshSegments) _returnvalue_3)))

(fn Setup
  (for _array_element (Variables|Default|GetLinks)
    (Physics|SetPhysicsLinearVelocity _array_element "0, 0, 0" false "None")
    (Class|PrimitiveComponent|SetPhysicsAngularVelocityinDegrees _array_element "0, 0, 0" false "None")
    (Development|PrintString "1")))